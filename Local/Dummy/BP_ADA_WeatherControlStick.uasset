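; Placeable Conan weather control stick that creates a resizable, high-priority climate zone with a fixed weather setting around itself.
; SetSize scales the trigger box and spawns or rescales a BP_WeatherClimateArea, which is destroyed on EndPlay.
; Local players entering the box have Ultra Dynamic Sky's time of day forced to zero.
; Owners edit size through a radial-menu popup; the server persists DynamicSize and OnRep reapplies it.
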(event `self.ReceiveBeginPlay`
  ;[1 1 0.5] (Both) BeginPlay
  (`parent.ReceiveBeginPlay`)
  (`self.SetSize` (`self.DynamicSize`)))

(event `self.ReceiveEndPlay`
  (params (EndPlayReason :type "EEndPlayReason Enum" :default "Destroyed"))
  ;[1 1 0.5] (Both) EndPlay
  (`parent.ReceiveEndPlay` EndPlayReason)
  (`self.K2_DestroyActor` (`self.WeatherClimateArea`)))

(event `self.Box.OnComponentBeginOverlap`
  (params (OverlappedComponent :type "PrimitiveComponent Object Reference") (OtherActor :type "Actor Object Reference") (OtherComp :type "PrimitiveComponent Object Reference") (OtherBodyIndex :type Integer) (bFromSweep :type Boolean) (SweepResult :type "HitResult Structure (by ref)"))
  ;[0.5 1 1] (Client) OnOverlapBegin
  (if (`Controller.IsLocalPlayerController` (`/Game/Characters/FuncomFunctionLibrary.GetControllerFromActor` OtherActor))
    (bind _outactors (`GameplayStatics.GetAllActorsOfClass` "/Game/Marketplace/UltraDynamicSky/Blueprints/Ultra_Dynamic_Sky_BP.Ultra_Dynamic_Sky_BP_C"))
    (bind _item (`KismetArrayLibrary.Array_Get` _outactors))
    (`/Engine/EditorBlueprintResources/StandardMacros.IsValid` _item
      (:`Is Valid`
        (`/Game/Marketplace/UltraDynamicSky/Blueprints/Ultra_Dynamic_Sky_BP.Editor_ForceTimeOfDay` _item 0.0)))))

(event `InteractableInterface.InteractableMenu`
  (params (RadialMenu :type "RadialMenu Object Reference") (HitIndex :type Integer))
  ;[0.5 1 1] (Client) Handle Menu Item
  (`parent.InteractableMenu` RadialMenu HitIndex)
  (if (`self.IsOwner` (`Controller.K2_GetPawn` (`UserWidget.GetOwningPlayer` RadialMenu)))
    (bind _returnvalue (`RadialMenu.AddItem` RadialMenu "ADA Config" (`/Game/Characters/SurvivalFunctionLibrary.GetBuildableObjectName` self) "/Game/Mods/AmunetDungeonAssets/UI/T_icon_edit.T_icon_edit" "None" 0))
    (add `RadialMenuEntry.SignalClicked` _returnvalue (delegate `ClientClickedEdit`))))

(event `ClientClickedEdit`
  (params (menuEntry :type "RadialMenuEntry Object Reference"))
  ;[0.5 1 1] (Client) Handle Menu Item
  (`self.ClientLoadPopup`))

(event `ClientLoadPopup`
  ;[0.5 1 1] (Client) Trigger Configure
  (bind _returnvalue (`GUIModuleController.ActivateModule` (`GUIModuleController.GetGUIModuleController`) "TriggerConfig" true false))
  (bind _asw_ada_config_trigger (cast `/Game/Mods/AmunetDungeonAssets/UI/W_ADA_ConfigTrigger` _returnvalue))
  (`/Game/Mods/AmunetDungeonAssets/UI/W_ADA_ConfigTrigger.ConfigTrigger` _asw_ada_config_trigger self "" false "" false 0 false 0 false 0 false 0 false 0 false 0 false 0.0 false (`self.DynamicSize`) true 0.0 false 0 false "" false))

(event `/Game/Mods/AmunetDungeonAssets/ADA_TriggerInterface.ConfigTrigger`
  (params (Name :type String) (NameSub :type String) (ValueTrigger :type Integer) (ValueUp :type Integer) (ValueDown :type Integer) (ValueMask :type Integer) (ValueItemId :type Integer) (ValueItemQuantity :type Integer) (ValueDelay :type "Float (single-precision)") (ValueSize :type "Float (single-precision)") (ValueDamage :type "Float (single-precision)") (ValueVariant :type Integer) (ValueSequence :type String))
  ;[1 0.5 0.5] (Server) Trigger Configure
  (set `self.DynamicSize` ValueSize)
  (`PersistenceComponent.SetDirty` (`self.ConanBuildingPersistence`) true 5.0))

(fn `OnRep_Size`
  (`self.SetSize` (`self.DynamicSize`)))

(fn `SetSize`
  (params (Size :type "Float (double-precision)"))
  (bind _returnvalue (* Size 168.0))
  (bind _weatherclimatearea (`self.WeatherClimateArea`))
  (bind _box (`self.Box`))
  (bind _returnvalue_2 (/ _returnvalue 1000.0))
  (bind _returnvalue_3 (`KismetMathLibrary.MakeVector` _returnvalue_2 _returnvalue_2 0.84))
  (`SceneComponent.SetWorldScale3D` _box (`KismetMathLibrary.MakeVector` _returnvalue _returnvalue 840.0))
  (`/Engine/EditorBlueprintResources/StandardMacros.IsValid` _weatherclimatearea
    (:`Is Valid`
      (`SceneComponent.SetWorldScale3D` (`/Game/Systems/Weather/BP_WeatherClimateArea.DefaultSceneRoot` _weatherclimatearea) _returnvalue_3))
    (:`Is Not Valid`
      (bind _returnvalue_4 (`|SpawnActorFromClass` "/Game/Systems/Weather/BP_WeatherClimateArea.BP_WeatherClimateArea_C" (`KismetMathLibrary.MakeTransform` (`SceneComponent.K2_GetComponentLocation` _box) (`SceneComponent.K2_GetComponentRotation` _box) _returnvalue_3) "AlwaysSpawn" "OverrideRootScale"))
      (bind _output_get (set `self.WeatherClimateArea` _returnvalue_4))
      (set `/Game/Systems/Weather/BP_WeatherClimateArea.WeatherClimate` "NewEnumerator4" _output_get)
      (set `/Game/Systems/Weather/BP_WeatherClimateArea.DisabledWeatherTimeOfDay` 0.0 _output_get)
      (set `/Game/Systems/Weather/BP_WeatherClimateArea.DisabledWeatherSunInclination` -1.0 _output_get)
      (set `/Game/Systems/Weather/BP_WeatherClimateArea.DisabledWeatherSunAngle` 90.0 _output_get)
      (set `/Game/Systems/Weather/BP_WeatherClimateArea.Priority` 1000 _output_get))))

(fn `UserConstructionScript`
  (`parent.UserConstructionScript`))