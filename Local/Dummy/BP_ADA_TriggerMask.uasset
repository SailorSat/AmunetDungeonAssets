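; Amunet Dungeon Assets buildable trigger that combines incoming trigger values into a bitmask, like a multi-input logic gate.
; On the server it registers with the ModController; values of 2+ OR bits into the stored state, values of -2 or lower XOR them.
; It then fires its sub-trigger with the Down value on an exact mask match, otherwise Up.
; Owners edit settings through a radial-menu popup; unregistering on EndPlay is unwired.
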(event `/Game/Mods/AmunetDungeonAssets/ADA_TriggerInterface.ActivateTrigger`
  (params (Name :type String) (Value :type Integer) (Component :type "PrimitiveComponent Object Reference") (Instigator :type "Controller Object Reference") (HitIndex :type Integer))
  (bind _returnvalue (`KismetMathLibrary.Abs_Int` Value))
  (bind _tempvalue (`self.TempValue`))
  (bind _triggername (`self.TriggerName`))
  (if (== _triggername Name)
    (if (== (`self.TriggerSubName`) _triggername)
      _
      (elif (<= Value -2)
        (set `self.TempValue` (`KismetMathLibrary.Xor_IntInt` _returnvalue _tempvalue))
        (`/Game/Mods/AmunetDungeonAssets/AmunetDungeonAssets_ModController.ActivateTrigger` (`self.ModController`) (`self.TriggerSubName`) (select `bool` (== (stale _output_get) (`self.TriggerMask`)) :`false` (`self.TriggerValueUp`) :`true` (`self.TriggerValueDown`)) Component Instigator HitIndex :!label _label)
        (elif (>= Value 2)
          (bind _output_get (set `self.TempValue` (`KismetMathLibrary.Or_IntInt` _returnvalue _tempvalue)))
          (goto _label))))))

(event `self.ReceiveBeginPlay`
  ;[1 1 1] Handle (Un)registering
  (`parent.ReceiveBeginPlay`)
  (if (`KismetSystemLibrary.IsServer`)
    (if (not (== (`KismetMathLibrary.MakeVector` 0.0) (`self.K2_GetActorLocation` self)))
      (bind _outactors (`GameplayStatics.GetAllActorsOfClass` "/Game/Mods/AmunetDungeonAssets/AmunetDungeonAssets_ModController.AmunetDungeonAssets_ModController_C"))
      (bind _output_get (set `self.ModController` (`KismetArrayLibrary.Array_Get` _outactors)))
      (message `/Game/Mods/AmunetDungeonAssets/ADA_TriggerInterface.RegisterTrigger` _output_get self))))

(event `self.ReceiveEndPlay`
  (params (EndPlayReason :type "EEndPlayReason Enum" :default "Destroyed"))
  ;[1 1 1] Handle (Un)registering
  (`parent.ReceiveEndPlay` EndPlayReason))

(event `InteractableInterface.InteractableMenu`
  (params (RadialMenu :type "RadialMenu Object Reference") (HitIndex :type Integer))
  ;[0.5 1 1] (Client) Handle Menu Item
  (`parent.InteractableMenu` RadialMenu HitIndex)
  (if (`self.IsOwner` (`Controller.K2_GetPawn` (`UserWidget.GetOwningPlayer` RadialMenu)))
    (bind _returnvalue (`RadialMenu.AddItem` RadialMenu "ADA Config" (`/Game/Characters/SurvivalFunctionLibrary.GetBuildableObjectName` self) "/Game/Mods/AmunetDungeonAssets/UI/T_icon_edit.T_icon_edit" "None" 0))
    (add `RadialMenuEntry.SignalClicked` _returnvalue (delegate `ClientClickedEdit`))))

(event `ClientClickedEdit`
  (params (menuEntry :type "RadialMenuEntry Object Reference"))
  ;[0.5 1 1] (Client) Handle Menu Item
  (`self.ClientLoadPopup`))

(event `/Game/Mods/AmunetDungeonAssets/ADA_TriggerInterface.ConfigTrigger`
  (params (Name :type String) (NameSub :type String) (ValueTrigger :type Integer) (ValueUp :type Integer) (ValueDown :type Integer) (ValueMask :type Integer) (ValueItemId :type Integer) (ValueItemQuantity :type Integer) (ValueDelay :type "Float (single-precision)") (ValueSize :type "Float (single-precision)") (ValueDamage :type "Float (single-precision)") (ValueVariant :type Integer) (ValueSequence :type String))
  ;[1 0.5 0.5] (Server) Trigger Configure
  (set `self.TriggerName` Name)
  (set `self.TriggerSubName` NameSub)
  (set `self.TriggerValueUp` ValueUp)
  (set `self.TriggerValueDown` ValueDown)
  (set `self.TriggerMask` ValueMask)
  (`PersistenceComponent.SetDirty` (`self.ConanBuildingPersistence`) true 5.0))

(event `ClientLoadPopup`
  ;[0.5 1 1] (Client) Trigger Configure
  (bind _returnvalue (`GUIModuleController.ActivateModule` (`GUIModuleController.GetGUIModuleController`) "TriggerConfig" true false))
  (bind _asw_ada_config_trigger (cast `/Game/Mods/AmunetDungeonAssets/UI/W_ADA_ConfigTrigger` _returnvalue))
  (`/Game/Mods/AmunetDungeonAssets/UI/W_ADA_ConfigTrigger.ConfigTrigger` _asw_ada_config_trigger self (`self.TriggerName`) true (`self.TriggerSubName`) true 0 false (`self.TriggerValueUp`) true (`self.TriggerValueDown`) true (`self.TriggerMask`) true 0 false 0 false 0.0 false 0.0 false 0.0 false 0 false "" false))

(fn `OnRep_TriggerName`)

(fn `UserConstructionScript`
  (`parent.UserConstructionScript`))