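; BP_ADA_AcidControlStick is an actor with a Box trigger volume that applies an acid bath buff to actors inside it.
; On the server, a begin overlap adds BP_AC_Buff_AcidBath at zero potency through the other actor's 00_BP_AC_BuffSystem component, and an end overlap removes it.
; Actors without that component are ignored, and the construction script only calls its parent.
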(event `self.Box.OnComponentBeginOverlap`
  (params (OverlappedComponent :type "PrimitiveComponent Object Reference") (OtherActor :type "Actor Object Reference") (OtherComp :type "PrimitiveComponent Object Reference") (OtherBodyIndex :type Integer) (bFromSweep :type Boolean) (SweepResult :type "HitResult Structure (by ref)"))
  (bind _returnvalue (`self.K2_GetComponentsByClass` OtherActor "/Game/Systems/Buffs/00_BP_AC_BuffSystem.00_BP_AC_BuffSystem_C"))
  (if (`KismetSystemLibrary.IsServer`)
    (if (> (`KismetArrayLibrary.Array_Length` _returnvalue) 0)
      (`/Game/Systems/Buffs/00_BP_AC_BuffSystem.AddBuff` (`KismetArrayLibrary.Array_Get` _returnvalue) "/Game/Systems/Buffs/Damage_Percent/BP_AC_Buff_AcidBath.BP_AC_Buff_AcidBath_C" 0 null))))

(event `self.Box.OnComponentEndOverlap`
  (params (OverlappedComponent :type "PrimitiveComponent Object Reference") (OtherActor :type "Actor Object Reference") (OtherComp :type "PrimitiveComponent Object Reference") (OtherBodyIndex :type Integer))
  (bind _returnvalue (`self.K2_GetComponentsByClass` OtherActor "/Game/Systems/Buffs/00_BP_AC_BuffSystem.00_BP_AC_BuffSystem_C"))
  (if (`KismetSystemLibrary.IsServer`)
    (if (> (`KismetArrayLibrary.Array_Length` _returnvalue) 0)
      (`/Game/Systems/Buffs/00_BP_AC_BuffSystem.RemoveBuff` (`KismetArrayLibrary.Array_Get` _returnvalue) "/Game/Systems/Buffs/Damage_Percent/BP_AC_Buff_AcidBath.BP_AC_Buff_AcidBath_C"))))

(fn `UserConstructionScript`
  (`parent.UserConstructionScript`))