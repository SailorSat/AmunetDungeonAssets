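; Buildable trigger relay for the Amunet Dungeon Assets mod that turns one incoming trigger into a timed up/down pulse.
; On the server it registers with the mod controller and, when its name arrives with value -1, fires the sub-trigger's up value, then its down value after a delay.
; An active flag blocks repeat up signals, and matching input and output names are ignored.
; Owners configure it through a radial-menu Edit popup, with changes marked for persistence.
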(event `/Game/Mods/AmunetDungeonAssets/AmunetDungeonAssets_TriggerInterface.ActivateTrigger`
  (params (Name :type String) (Value :type Integer) (Component :type "PrimitiveComponent Object Reference") (Instigator :type "Controller Object Reference") (HitIndex :type Integer))
  (bind _triggername (`self.TriggerName`))
  (`/Game/Systems/BP_MacroGlobal.And+Branch` (`KismetStringLibrary.EqualEqual_StrStr` _triggername Name) (== Value -1)
    (:`True`
      (if (not (`KismetStringLibrary.EqualEqual_StrStr` (`self.TriggerSubName`) _triggername))
        (if (not (`self.TriggerActive`))
          (set `self.TriggerActive` true)
          (`/Game/Mods/AmunetDungeonAssets/AmunetDungeonAssets_ModController.ActivateTrigger` (`self.ModController`) (`self.TriggerSubName`) (`self.TriggerValueUp`) Component Instigator HitIndex))
        (`KismetSystemLibrary.Delay` (`self.TriggerDelay`))
        (set `self.TriggerActive` false)
        (`/Game/Mods/AmunetDungeonAssets/AmunetDungeonAssets_ModController.ActivateTrigger` (`self.ModController`) (`self.TriggerSubName`) (`self.TriggerValueDown`) Component Instigator HitIndex)))))

(event `self.ReceiveBeginPlay`
  ;[1 1 1] Handle (Un)registering
  (if (`KismetSystemLibrary.IsServer`)
    (if (not (== (`KismetMathLibrary.MakeVector` 0.0) (`self.K2_GetActorLocation` self)))
      (bind _outactors (`GameplayStatics.GetAllActorsOfClass` "/Game/Mods/AmunetDungeonAssets/AmunetDungeonAssets_ModController.AmunetDungeonAssets_ModController_C"))
      (bind _output_get (set `self.ModController` (`KismetArrayLibrary.Array_Get` _outactors)))
      (message `/Game/Mods/AmunetDungeonAssets/AmunetDungeonAssets_TriggerInterface.RegisterTrigger` _output_get self))))

(event `self.ReceiveEndPlay`
  (params (EndPlayReason :type "EEndPlayReason Enum" :default "Destroyed"))
  (bind _modcontroller (`self.ModController`))
  ;[1 1 1] Handle (Un)registering
  (`/Game/Systems/BP_MacroGlobal.IsValid+Branch` _modcontroller (`KismetSystemLibrary.IsServer`)
    (:`True`
      (message `/Game/Mods/AmunetDungeonAssets/AmunetDungeonAssets_TriggerInterface.UnregisterTrigger` _modcontroller self))))

(event `InteractableInterface.InteractableMenu`
  (params (RadialMenu :type "RadialMenu Object Reference") (HitIndex :type Integer))
  ;[0.5 1 1] (Client) Handle Menu Item
  (`parent.InteractableMenu` RadialMenu HitIndex)
  (if (`self.IsOwner` (`Controller.K2_GetPawn` (`UserWidget.GetOwningPlayer` RadialMenu)))
    (bind _returnvalue (`RadialMenu.AddItem` RadialMenu "Edit" (`/Game/Characters/SurvivalFunctionLibrary.GetBuildableObjectName` self) "/Game/UI/Textures/GUIs/Guild/T_EditButton.T_EditButton" "None" 0))
    (add `RadialMenuEntry.SignalClicked` _returnvalue (delegate `ClientClickedEdit`))))

(event `ClientClickedEdit`
  (params (menuEntry :type "RadialMenuEntry Object Reference"))
  ;[0.5 1 1] (Client) Handle Menu Item
  (`self.ClientLoadPopup`))

(event `/Game/Mods/AmunetDungeonAssets/AmunetDungeonAssets_TriggerInterface.ConfigTrigger`
  (params (Name :type String) (NameSub :type String) (ValueTrigger :type Integer) (ValueUp :type Integer) (ValueDown :type Integer) (ValueMask :type Integer) (ValueItemId :type Integer) (ValueItemQuantity :type Integer) (ValueDelay :type "Float (single-precision)"))
  ;[1 0.5 0.5] (Server) Trigger Configure
  (set `self.TriggerName` Name)
  (set `self.TriggerSubName` NameSub)
  (set `self.TriggerValueUp` ValueUp)
  (set `self.TriggerValueDown` ValueDown)
  (set `self.TriggerDelay` ValueDelay)
  (`PersistenceComponent.SetDirty` (`self.ConanBuildingPersistence`) true 5.0))

(event `ClientLoadPopup`
  ;[0.5 1 1] (Client) Trigger Configure
  (bind _returnvalue (`GUIModuleController.ActivateModule` (`GUIModuleController.GetGUIModuleController`) "TriggerConfig" true false))
  (bind _asw_ada_config_trigger (cast `/Game/Mods/AmunetDungeonAssets/UI/W_ADA_ConfigTrigger` _returnvalue))
  (`/Game/Mods/AmunetDungeonAssets/UI/W_ADA_ConfigTrigger.ConfigTrigger` _asw_ada_config_trigger self (`self.TriggerName`) (`self.TriggerSubName`) true 0 false (`self.TriggerValueUp`) true (`self.TriggerValueDown`) true 0 false 0 false 0 false (`self.TriggerDelay`) true))

(fn `OnRep_TriggerName`)

(fn `UserConstructionScript`
  (`parent.UserConstructionScript`))