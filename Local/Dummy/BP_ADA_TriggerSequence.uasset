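; BP_ADA_TriggerSequence is a placeable trigger relay that fires a numbered sequence of named triggers through the Amunet Dungeon Assets mod controller.
; It registers by name on the server; value 1 starts a looping timer, and value 0 resets it with zero time, stopping it.
; Each tick activates "SubName_counter", wrapping the counter after TriggerMask.
; Owners configure it via a radial-menu popup, and server-side edits re-register and mark persistence dirty.
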(event `self.ReceiveBeginPlay`
  ;[1 1 1] Handle (Un)registering
  (`parent.ReceiveBeginPlay`)
  (if (`KismetSystemLibrary.IsServer`)
    (bind _outactors (`GameplayStatics.GetAllActorsOfClass` "/Game/Mods/AmunetDungeonAssets/AmunetDungeonAssets_ModController.AmunetDungeonAssets_ModController_C"))
    (bind _output_get (set `self.ModController` (`KismetArrayLibrary.Array_Get` _outactors)))
    (`/Game/ModsShared/AmunetDungeonAssets/Interfaces/ADA_I_TriggerController.RegisterTriggerTarget` _output_get self (`self.TriggerName`))))

(event `self.ReceiveEndPlay`
  (params (EndPlayReason :type "EEndPlayReason Enum" :default "Destroyed"))
  ;[1 1 1] Handle (Un)registering
  (`parent.ReceiveEndPlay` EndPlayReason)
  (`/Game/Systems/BP_MacroGlobal.IsValid+Branch` (`self.ModController`) (`KismetSystemLibrary.IsServer`)
    (:`True`
      (`/Game/ModsShared/AmunetDungeonAssets/Interfaces/ADA_I_TriggerController.UnregisterTriggerTarget` (stale `self.ReceiveBeginPlay` _output_get) self (`self.TriggerName`)))))

(event `/Game/ModsShared/AmunetDungeonAssets/Interfaces/ADA_I_TriggerTarget.ActivateTrigger`
  (params (Value :type Integer) (Component :type "PrimitiveComponent Object Reference") (Instigator :type "Controller Object Reference") (HitIndex :type Integer))
  (switch `int` Value
    (:`0`
      (`KismetSystemLibrary.K2_SetTimerDelegate` (delegate `AdvanceSequence`) 0.0))
    (:`1`
      (`KismetSystemLibrary.K2_SetTimerDelegate` (delegate `AdvanceSequence`) (`self.TriggerDelay`) true))))

(event `InteractableInterface.InteractableMenu`
  (params (RadialMenu :type "RadialMenu Object Reference") (HitIndex :type Integer))
  ;[0.5 1 1] (Client) Handle Menu Item
  (`parent.InteractableMenu` RadialMenu HitIndex)
  (if (`self.IsOwner` (`Controller.K2_GetPawn` (`UserWidget.GetOwningPlayer` RadialMenu)))
    (bind _returnvalue (`RadialMenu.AddItem` RadialMenu "ADA Config" (`/Game/Systems/Building/BuildingFunctionLibrary.GetBuildableObjectName` self) "/Game/Mods/AmunetDungeonAssets/UI/T_icon_edit.T_icon_edit" "None" 0))
    (add `RadialMenuEntry.SignalClicked` _returnvalue (delegate `ClientClickedEdit`))))

(event `AdvanceSequence`
  (`/Game/ModsShared/AmunetDungeonAssets/Interfaces/ADA_I_TriggerController.ActivateTriggerTarget` (`self.ModController`) (`KismetStringLibrary.Concat_StrStr` (`self.TriggerSubName`) "_" (`KismetStringLibrary.Conv_IntToString` (`self.TempCounter`))) (`self.TriggerValue`) (stale `/Game/ModsShared/AmunetDungeonAssets/Interfaces/ADA_I_TriggerTarget.ActivateTrigger` Component) (stale `/Game/ModsShared/AmunetDungeonAssets/Interfaces/ADA_I_TriggerTarget.ActivateTrigger` Instigator) (stale `/Game/ModsShared/AmunetDungeonAssets/Interfaces/ADA_I_TriggerTarget.ActivateTrigger` HitIndex))
  (bind _result (`/Engine/EditorBlueprintResources/StandardMacros.IncrementInt` (`self.TempCounter`))
    (:`  `
      (if (> _result (`self.TriggerMask`))
        (set `self.TempCounter` 0)))))

(event `ClientClickedEdit`
  (params (menuEntry :type "RadialMenuEntry Object Reference"))
  ;[0.5 1 1] (Client) Handle Menu Item
  (`self.ClientLoadPopup`))

(event `/Game/ModsShared/AmunetDungeonAssets/Interfaces/ADA_I_TriggerTarget.ConfigTrigger`
  (params (Name :type String) (NameSub :type String) (ValueTrigger :type Integer) (ValueUp :type Integer) (ValueDown :type Integer) (ValueMask :type Integer) (ValueItemId :type Integer) (ValueItemQuantity :type Integer) (ValueDelay :type "Float (single-precision)") (ValueSize :type "Float (single-precision)") (ValueDamage :type "Float (single-precision)") (ValueVariant :type Integer) (ValueSequence :type String))
  ;[1 0.5 0.5] (Server) Trigger Configure
  (`/Game/ModsShared/AmunetDungeonAssets/Interfaces/ADA_I_TriggerController.UpdateTriggerTarget` (`self.ModController`) self (`self.TriggerName`) Name)
  (set `self.TriggerName` Name)
  (set `self.TriggerSubName` NameSub)
  (set `self.TriggerValue` ValueTrigger)
  (set `self.TriggerMask` ValueItemQuantity)
  (set `self.TriggerDelay` ValueDelay)
  (`PersistenceComponent.SetDirty` (`self.ConanBuildingPersistence`) true 5.0))

(event `ClientLoadPopup`
  (bind _triggermask (`self.TriggerMask`))
  ;[0.5 1 1] (Client) Trigger Configure
  (bind _returnvalue (`GUIModuleController.ActivateModule` (`GUIModuleController.GetGUIModuleController`) "TriggerConfig" true false))
  (bind _asw_ada_config_trigger (cast `/Game/Mods/AmunetDungeonAssets/UI/W_ADA_ConfigTrigger` _returnvalue))
  (`/Game/Mods/AmunetDungeonAssets/UI/W_ADA_ConfigTrigger.ConfigTrigger` _asw_ada_config_trigger self (`self.TriggerName`) true (`self.TriggerSubName`) true (`self.TriggerValue`) true 0 false 0 false _triggermask false 0 false _triggermask true (`self.TriggerDelay`) true 0.0 false 0.0 false 0 false "" false))

(fn `OnRep_TriggerName`)

(fn `UserConstructionScript`
  (`parent.UserConstructionScript`))