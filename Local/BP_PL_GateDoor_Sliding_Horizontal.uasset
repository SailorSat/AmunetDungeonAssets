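; Two-panel sliding gate door for Amunet Dungeon Assets, opened, closed or toggled by named trigger messages.
; The server registers it with the mod controller and matching messages set DoorState, while owners edit the trigger name through a radial-menu popup.
; Overridden door events slide both meshes apart or together on one timeline.
; Panels stop affecting navigation while moving, then a retry timer nudges blocking NPCs clear before restoring it.
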(event `self.ClosedToOpenNormal`
  ;[1 0.6413 0.1882] Override Door Events to include second door.
  ;;[0.02499 0.09524 0.16] Normal Direction
  (`self.SetGateDoorsNotAffectNavigation` :!label _label)
  (`GameplayStatics.PlaySoundAtLocation` (`self.SoundToPlayOpen`) (`self.K2_GetActorLocation`))
  (bind (_direction _rotation) (`Timeline|Timeline_1` :!label _label_2)
    (:`Update`
      ;;;[0.02499 0.09524 0.16] Door #1
      (`SceneComponent.K2_SetRelativeLocation` (`self.StaticMesh`) (`KismetMathLibrary.MakeVector` (* _rotation 128.0) 0.0 -248.0) false false)
      ;;;[0.02499 0.09524 0.16] Door #2
      (`SceneComponent.K2_SetRelativeLocation` (`self.StaticMesh1`) (`KismetMathLibrary.MakeVector` (* _rotation -128.0) 0.0 -248.0) false false))
    (:`Finished`
      (set `self.IsLastOpenCloseFinished` true)
      (`self.ChangeNavMeshAreaGateDoor`))))

(event `self.ClosedToOpenReverse`
  ;[1 0.6413 0.1882] Override Door Events to include second door.
  ;;[0.02499 0.09524 0.16] Normal Direction
  (goto _label))

(event `self.OpenNormalToClosed`
  ;[1 0.6413 0.1882] Override Door Events to include second door.
  ;;[0.02499 0.09524 0.16] Normal Direction
  (`self.SetGateDoorsNotAffectNavigation` :!label _label_3)
  (`GameplayStatics.PlaySoundAtLocation` (`self.SoundToPlayClose`) (`self.K2_GetActorLocation`))
  (goto _label_2 :!via `Reverse`))

(event `self.OpenReversedToClosed`
  ;[1 0.6413 0.1882] Override Door Events to include second door.
  ;;[0.02499 0.09524 0.16] Normal Direction
  (goto _label_3))

(event `self.ReceiveBeginPlay`
  ;[1 0.5 0.5] Handle (Un)registering
  (`parent.ReceiveBeginPlay`)
  (if (`KismetSystemLibrary.IsServer`)
    (bind _outactors (`GameplayStatics.GetAllActorsOfClass` "/Game/Mods/AmunetDungeonAssets/AmunetDungeonAssets_ModController.AmunetDungeonAssets_ModController_C"))
    (bind _output_get (set `self.ModController` (`KismetArrayLibrary.Array_Get` _outactors)))
    (message `/Game/Mods/AmunetDungeonAssets/ADA_TriggerInterface.RegisterTrigger` _output_get self)))

(event `self.ReceiveEndPlay`
  (params (EndPlayReason :type "EEndPlayReason Enum" :default "Destroyed"))
  ;[1 0.5 0.5] Handle (Un)registering
  (`parent.ReceiveEndPlay` EndPlayReason)
  (`/Game/Systems/BP_MacroGlobal.IsValid+Branch` (`self.ModController`) (`KismetSystemLibrary.IsServer`)
    (:`True`
      (message `/Game/Mods/AmunetDungeonAssets/ADA_TriggerInterface.UnregisterTrigger` (stale `self.ReceiveBeginPlay` _output_get) self))))

(event `/Game/Mods/AmunetDungeonAssets/ADA_TriggerInterface.ActivateTrigger`
  (params (Name :type String) (Value :type Integer) (Component :type "PrimitiveComponent Object Reference") (Instigator :type "Controller Object Reference") (HitIndex :type Integer))
  (bind _doorstate (`self.DoorState`))
  ;[1 0.5 0.5] (Server) Activate Trigger
  (if (== (`self.TriggerName`) Name)
    (switch `int` Value
      (:`-1`
        (switch `/Game/Systems/Building/Placeables/EDoorState` _doorstate
          (:`NewEnumerator0`
            (set `self.DoorState` "NewEnumerator1" :!label _label_4))
          (:`NewEnumerator1`
            (set `self.DoorState` "NewEnumerator0" :!label _label_5))
          (:`NewEnumerator2`
            (goto _label_5))))
      (:`0`
        (switch `/Game/Systems/Building/Placeables/EDoorState` _doorstate
          (:`NewEnumerator1`
            (goto _label_5))
          (:`NewEnumerator2`
            (goto _label_5))))
      (:`1`
        (switch `/Game/Systems/Building/Placeables/EDoorState` _doorstate
          (:`NewEnumerator0`
            (goto _label_4)))))))

(event `InteractableInterface.InteractableMenu`
  (params (RadialMenu :type "RadialMenu Object Reference") (HitIndex :type Integer))
  ;[0.5 1 1] (Client) Handle Menu Item
  (`parent.InteractableMenu` RadialMenu HitIndex)
  (if (`self.IsOwner` (`Controller.K2_GetPawn` (`UserWidget.GetOwningPlayer` RadialMenu)))
    (bind _returnvalue (`RadialMenu.AddItem` RadialMenu "ADA Config" (`/Game/Characters/SurvivalFunctionLibrary.GetBuildableObjectName` self) "/Game/Mods/AmunetDungeonAssets/UI/T_icon_edit.T_icon_edit" "None" 0))
    (add `RadialMenuEntry.SignalClicked` _returnvalue (delegate `ClientClickedEdit`))))

(event `ClientClickedEdit`
  (params (menuEntry :type "RadialMenuEntry Object Reference"))
  ;[0.5 1 1] (Client) Handle Menu Item
  (`self.ClientLoadPopup`))

(event `ClientLoadPopup`
  ;[0.5 1 1] (Client) Trigger Configure
  (bind _returnvalue (`GUIModuleController.ActivateModule` (`GUIModuleController.GetGUIModuleController`) "TriggerConfig" true false))
  (bind _asw_ada_config_trigger (cast `/Game/Mods/AmunetDungeonAssets/UI/W_ADA_ConfigTrigger` _returnvalue))
  (`/Game/Mods/AmunetDungeonAssets/UI/W_ADA_ConfigTrigger.ConfigTrigger` _asw_ada_config_trigger self (`self.TriggerName`) true "" false 0 false 0 false 0 false 0 false 0 false 0 false 0.0 false 0.0 false 0.0 false 0 false "" false))

(event `/Game/Mods/AmunetDungeonAssets/ADA_TriggerInterface.ConfigTrigger`
  (params (Name :type String) (NameSub :type String) (ValueTrigger :type Integer) (ValueUp :type Integer) (ValueDown :type Integer) (ValueMask :type Integer) (ValueItemId :type Integer) (ValueItemQuantity :type Integer) (ValueDelay :type "Float (single-precision)") (ValueSize :type "Float (single-precision)") (ValueDamage :type "Float (single-precision)") (ValueVariant :type Integer) (ValueSequence :type String))
  ;[1 0.5 0.5] (Server) Trigger Configure
  (set `self.TriggerName` Name)
  (`PersistenceComponent.SetDirty` (`self.ConanBuildingPersistence`) true 5.0))

(fn `ChangeNavMeshAreaGateDoor`
  (bind _canchangenavmeshcheckergatedoorl (`self.CanChangeNavMeshCheckerGateDoorL`))
  (bind _canchangenavmeshcheckergatedoorr (`self.CanChangeNavMeshCheckerGateDoorR`))
  ;[1 1 1] Change the NavArea after the two gatedoors have been opened/closed. Make sure no overlapping with NPCs before changing. So no NPC will get stuck in  the gatedoor geomerty or be forced off navmesh.
  (bind (_outactors _returnvalue) (`KismetSystemLibrary.ComponentOverlapActors` _canchangenavmeshcheckergatedoorl (`SceneComponent.K2_GetComponentToWorld` _canchangenavmeshcheckergatedoorl) (`|MakeArray` "ObjectTypeQuery3" :!type "EObjectTypeQuery Enum") "/Game/Characters/NPCs/Humanoid/BaseHumanoidNPC.BaseHumanoidNPC_C"))
  (if _returnvalue
    (for _array_element _outactors
      (bind _asconan_basic_aicontroller (cast `ConanBasicAIController` (`Pawn.GetController` (`Actor.Instigator` _array_element))))
      (`ConanBasicAIController.MoveToAvoidBlocking` _asconan_basic_aicontroller self))
    (bind _returnvalue_2 (`KismetSystemLibrary.K2_SetTimer` null "ChangeNavMeshAreaGateDoor" 0.1))
    (set `self.ChangeNavMeshTimerHandler` _returnvalue_2)
    (else
      (bind (_outactors_2 _returnvalue_3) (`KismetSystemLibrary.ComponentOverlapActors` _canchangenavmeshcheckergatedoorr (`SceneComponent.K2_GetComponentToWorld` _canchangenavmeshcheckergatedoorr) (`|MakeArray` "ObjectTypeQuery3" :!type "EObjectTypeQuery Enum") "/Game/Characters/NPCs/Humanoid/BaseHumanoidNPC.BaseHumanoidNPC_C"))
      (if _returnvalue_3
        (for _array_element_2 _outactors_2
          (bind _asconan_basic_aicontroller_2 (cast `ConanBasicAIController` (`Pawn.GetController` (`Actor.Instigator` _array_element_2))))
          (`ConanBasicAIController.MoveToAvoidBlocking` _asconan_basic_aicontroller_2 self))
        (bind _returnvalue_4 (`KismetSystemLibrary.K2_SetTimer` null "ChangeNavMeshAreaGateDoor" 0.1))
        (set `self.ChangeNavMeshTimerHandler` _returnvalue_4)
        (else
          (`self.SetCanEverAffectNavigation` (`self.StaticMesh`) true)
          (`self.SetCanEverAffectNavigation` (`self.StaticMesh1`) true)
          (`KismetSystemLibrary.K2_ClearAndInvalidateTimerHandle` (`self.ChangeNavMeshTimerHandler`)))))))

(fn `GiveJourney_VillageGates`
  (bind _staticmesh (`self.StaticMesh`))
  ;[0.62 0 0] Make sure this Journey Event can only happen on Trial, and not get triggered by building Brush.
  (if (`DreamworldBlueprints.IsInTrialMode`)
    (if (`KismetSystemLibrary.IsServer`)
      (if (not (`self.IsABrush`))
        ;[0.62 0 0] Check if overlapping with Village Gate Journey Marker.
        (set `PrimitiveComponent.bGenerateOverlapEvents` true _staticmesh)
        (`FuncomGenericLibrary.UpdateOverlaps` self)
        (if (> (`KismetArrayLibrary.Array_Length` (`PrimitiveComponent.GetOverlappingActors` _staticmesh "/Game/Systems/Progression/BP_ExilesJourney_GateLocation.BP_ExilesJourney_GateLocation_C")) 0)
          (set `PrimitiveComponent.bGenerateOverlapEvents` false (`self.StaticMesh`))
          ;[1 0.6413 0.1882] Add Journey Event if an overlap with Journey Marker was detected.
          (bind _asbase_game_mode_interface (cast `/Game/Systems/Interfaces/BaseGameModeInterface` (`GameplayStatics.GetGameMode`)))
          (bind _actor (`/Game/Systems/Interfaces/BaseGameModeInterface.Get Actor By UniqueID Interface` _asbase_game_mode_interface (`self.OwnerUniqueID`)))
          (`ExilesJourneyComponent.AddJourneyEvent` (`self.GetComponentByClass` _actor "/Game/Systems/Progression/BP_AC_ExilesJourney.BP_AC_ExilesJourney_C") "ReplaceVillageGates" (`self.K2_GetActorLocation`)))))))

(fn `InteractableGetUIModuleName`
  (returns (ReturnValue :type Name))
  (return "None"))

(fn `IsGateDoor`
  (returns (GateDoor :type Boolean))
  (return false))

(fn `SetGateDoorsNotAffectNavigation`
  (`self.SetCanEverAffectNavigation` (`self.StaticMesh`))
  (`self.SetCanEverAffectNavigation` (`self.StaticMesh1`)))

(fn `UserConstructionScript`
  (`parent.UserConstructionScript`))