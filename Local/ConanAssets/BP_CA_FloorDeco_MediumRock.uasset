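; Placeable medium rock floor decoration for Conan building, with an owner-selectable cliff material variant (moss, plain, Cimmeria, frost, jungle, snow, swamp).
; Owners get an "ADA Config" radial menu entry that opens the TriggerConfig GUI module on the client.
; The server-side ConfigTrigger stores DynamicVariant and marks building persistence dirty.
; SetVariant swaps the instanced mesh material from both the construction script and DynamicVariant's OnRep.
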(event `InteractableInterface.InteractableMenu`
  (params (RadialMenu :type "RadialMenu Object Reference") (HitIndex :type Integer))
  ;[0.5 1 1] (Client) Handle Menu Item
  (`parent.InteractableMenu` RadialMenu HitIndex)
  (if (`self.IsOwner` (`Controller.K2_GetPawn` (`UserWidget.GetOwningPlayer` RadialMenu)))
    (bind _returnvalue (`RadialMenu.AddItem` RadialMenu "ADA Config" (`/Game/Characters/SurvivalFunctionLibrary.GetBuildableObjectName` self) "/Game/Mods/AmunetDungeonAssets/UI/T_icon_edit.T_icon_edit" "None" 0))
    (add `RadialMenuEntry.SignalClicked` _returnvalue (delegate `ClientClickedEdit`))))

(event `ClientClickedEdit`
  (params (menuEntry :type "RadialMenuEntry Object Reference"))
  ;[0.5 1 1] (Client) Handle Menu Item
  (`self.ClientLoadPopup`))

(event `ClientLoadPopup`
  ;[0.5 1 1] (Client) Trigger Configure
  (bind _returnvalue (`GUIModuleController.ActivateModule` (`GUIModuleController.GetGUIModuleController`) "TriggerConfig" true false))
  (bind _asw_ada_config_trigger (cast `/Game/Mods/AmunetDungeonAssets/UI/W_ADA_ConfigTrigger` _returnvalue))
  (`/Game/Mods/AmunetDungeonAssets/UI/W_ADA_ConfigTrigger.ConfigTrigger` _asw_ada_config_trigger self "" false "" false 0 false 0 false 0 false 0 false 0 false 0 false 0.0 false 0.0 false 0.0 false (`self.DynamicVariant`) true "" false))

(event `/Game/Mods/AmunetDungeonAssets/ADA_TriggerInterface.ConfigTrigger`
  (params (Name :type String) (NameSub :type String) (ValueTrigger :type Integer) (ValueUp :type Integer) (ValueDown :type Integer) (ValueMask :type Integer) (ValueItemId :type Integer) (ValueItemQuantity :type Integer) (ValueDelay :type "Float (single-precision)") (ValueSize :type "Float (single-precision)") (ValueDamage :type "Float (single-precision)") (ValueVariant :type Integer) (ValueSequence :type String))
  ;[1 0.5 0.5] (Server) Trigger Configure
  (set `self.DynamicVariant` ValueVariant)
  (`PersistenceComponent.SetDirty` (`self.ConanBuildingPersistence`) true 5.0))

(fn `OnRep_DynamicVariant`
  (`self.SetVariant` (`self.DynamicVariant`)))

(fn `SetVariant`
  (params (Variant :type Integer))
  (bind _instancedstaticmesh (`self.InstancedStaticMesh`))
  (switch `int` Variant
    (:`Default`
      (`PrimitiveComponent.SetMaterial` _instancedstaticmesh 0 "/Game/Environment/Rocks/Materials/MI_cliff_04_Moss.MI_cliff_04_Moss"))
    (:`1`
      (`PrimitiveComponent.SetMaterial` _instancedstaticmesh 0 "/Game/Environment/Rocks/Materials/MI_cliff_04.MI_cliff_04"))
    (:`2`
      (`PrimitiveComponent.SetMaterial` _instancedstaticmesh 0 "/Game/Environment/Rocks/Materials/MI_cliff_04_Cimmeria.MI_cliff_04_Cimmeria"))
    (:`3`
      (`PrimitiveComponent.SetMaterial` _instancedstaticmesh 0 "/Game/Environment/Rocks/Materials/MI_cliff_04_M_Moss_Frost.MI_cliff_04_M_Moss_Frost"))
    (:`4`
      (`PrimitiveComponent.SetMaterial` _instancedstaticmesh 0 "/Game/Environment/Rocks/Materials/MI_cliff_04_jungle.MI_cliff_04_jungle"))
    (:`5`
      (`PrimitiveComponent.SetMaterial` _instancedstaticmesh 0 "/Game/Environment/Rocks/Materials/MI_cliff_04_M_Snow.MI_cliff_04_M_Snow"))
    (:`6`
      (`PrimitiveComponent.SetMaterial` _instancedstaticmesh 0 "/Game/Environment/Rocks/Materials/MI_cliff_04_Swamp.MI_cliff_04_Swamp"))))

(fn `UserConstructionScript`
  (`parent.UserConstructionScript`)
  (`self.SetVariant` (`self.DynamicVariant`)))