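; Pedestal wall button that players activate to fire a named trigger through the mod controller.
; Server-side interaction calls OnActivate, then passes the trigger name, value, instigator and hit details to ModController.
; OnActivate, marked for both server and client, plays a sound and runs a timeline that drives the point light's intensity.
; A completion flag ignores further presses until that timeline finishes.
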(event `OnActivate`
  ;[1 1 0.5] (Both) Animation and Sound
  (`self.PlaySound`)
  (bind (_direction _alpha) (`Timeline|Timeline_UpToDown` :!via `PlayFromStart`)
    (:`Update`
      (`LightComponent.SetIntensity` (`self.PointLight`) _alpha))
    (:`Finished`
      (set `self.IsLastAnimationFinished` true))))

(event `InteractableInterface.InteractableActivate`
  (params (Component :type "PrimitiveComponent Object Reference") (Instigator :type "PlayerController Object Reference") (HitIndex :type Integer) (TriggeredFromRadialWheel :type Boolean))
  ;[1 0.5 0.5] (Server) Interactable Activate
  (if (`self.IsLastAnimationFinished`)
    (set `self.IsLastAnimationFinished` false)
    (`self.OnActivate`)
    (`/Game/Mods/AmunetDungeonAssets/AmunetDungeonAssets_ModController.ActivateTrigger` (`self.ModController`) (`self.TriggerName`) (`self.TriggerValueTrigger`) Component Instigator HitIndex)))

(fn `UserConstructionScript`
  (`parent.UserConstructionScript`))