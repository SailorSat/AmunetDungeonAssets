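; Construction-time decoration Blueprint that scatters a small cluster of instanced meshes, named as rocks for wall decoration.
; After running the parent construction script, it loops to add instances to an InstancedStaticMesh component at random local offsets, spread widely along Y and narrowly on X and Z.
; Each instance gets a random yaw at unit scale.
; The random calls are unseeded, so the layout changes whenever the construction script reruns.
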(fn `UserConstructionScript`
  (`parent.UserConstructionScript`)
  (for _ (range 8)
    (`InstancedStaticMeshComponent.AddInstance` (`self.InstancedStaticMesh`) (`KismetMathLibrary.MakeTransform` (`KismetMathLibrary.MakeVector` (`KismetMathLibrary.RandomFloatInRange` -10.0 10.0) (`KismetMathLibrary.RandomFloatInRange` -168.0 168.0) (`KismetMathLibrary.RandomFloatInRange` -10.0 10.0)) (`KismetMathLibrary.MakeRotator` 0.0 0.0 (`KismetMathLibrary.RandomFloatInRange` 0.0 60.0))))))