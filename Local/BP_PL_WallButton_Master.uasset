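; Master Blueprint for a Conan Exiles placeable wall button that fires a named trigger in the Amunet Dungeon Assets mod.
; On interaction, the server plays the push animation and click via OnActivate, then forwards trigger name and value to the ModController, ignoring presses until the animation finishes.
; Owners get a radial-menu entry opening the TriggerConfig popup; ConfigTrigger stores edited values and marks building persistence dirty.
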(event `self.ReceiveBeginPlay`
  ;[1 0.5 0.5] (Server) BeginPlay
  (`parent.ReceiveBeginPlay`)
  (if (`KismetSystemLibrary.IsServer`)
    (bind _outactors (`GameplayStatics.GetAllActorsOfClass` "/Game/Mods/AmunetDungeonAssets/AmunetDungeonAssets_ModController.AmunetDungeonAssets_ModController_C"))
    (set `self.ModController` (`KismetArrayLibrary.Array_Get` _outactors))))

(event `OnActivate`
  ;[1 1 0.5] (Both) Animation and Sound
  (`self.PlaySound`)
  (bind (_direction _alpha) (`Timeline|Timeline_Push` :!via `PlayFromStart`)
    (:`Update`
      (`SceneComponent.K2_SetRelativeLocation` (`self.StaticMesh`) (`KismetMathLibrary.MakeVector` _alpha) false false))
    (:`Finished`
      (set `self.IsLastAnimationFinished` true))))

(event `InteractableInterface.InteractableActivate`
  (params (Component :type "PrimitiveComponent Object Reference") (Instigator :type "PlayerController Object Reference") (HitIndex :type Integer) (TriggeredFromRadialWheel :type Boolean))
  ;[1 0.5 0.5] (Server) Interactable Activate
  (if (`self.IsLastAnimationFinished`)
    (set `self.IsLastAnimationFinished` false)
    (`self.OnActivate`)
    (`/Game/ModsShared/AmunetDungeonAssets/Interfaces/ADA_I_TriggerController.ActivateTriggerTarget` (`self.ModController`) (`self.TriggerName`) (`self.TriggerValueTrigger`) Component Instigator HitIndex)))

(event `InteractableInterface.InteractableMenu`
  (params (RadialMenu :type "RadialMenu Object Reference") (HitIndex :type Integer))
  ;[0.5 1 1] (Client) Handle Menu Item
  (`parent.InteractableMenu` RadialMenu HitIndex)
  (if (`self.IsOwner` (`Controller.K2_GetPawn` (`UserWidget.GetOwningPlayer` RadialMenu)))
    (bind _returnvalue (`RadialMenu.AddItem` RadialMenu "ADA Config" (`/Game/Systems/Building/BuildingFunctionLibrary.GetBuildableObjectName` self) "/Game/Mods/AmunetDungeonAssets/UI/T_icon_edit.T_icon_edit" "None" 0))
    (add `RadialMenuEntry.SignalClicked` _returnvalue (delegate `ClientClickedEdit`))))

(event `ClientClickedEdit`
  (params (menuEntry :type "RadialMenuEntry Object Reference"))
  ;[0.5 1 1] (Client) Handle Menu Item
  (`self.ClientLoadPopup`))

(event `ClientLoadPopup`
  ;[0.5 1 1] (Client) Trigger Configure
  (bind _returnvalue (`GUIModuleController.ActivateModule` (`GUIModuleController.GetGUIModuleController`) "TriggerConfig" true false))
  (bind _asw_ada_config_trigger (cast `/Game/Mods/AmunetDungeonAssets/UI/W_ADA_ConfigTrigger` _returnvalue))
  (`/Game/Mods/AmunetDungeonAssets/UI/W_ADA_ConfigTrigger.ConfigTrigger` _asw_ada_config_trigger self "" false (`self.TriggerName`) true (`self.TriggerValueTrigger`) (`self.TriggerShowTrigger`) (`self.TriggerValueUp`) (`self.TriggerShowUp`) (`self.TriggerValueDown`) (`self.TriggerShowDown`) 0 false 0 false 0 false 0.0 false 0.0 false 0.0 false 0 false "" false))

(event `/Game/ModsShared/AmunetDungeonAssets/Interfaces/ADA_I_TriggerTarget.ConfigTrigger`
  (params (Name :type String) (NameSub :type String) (ValueTrigger :type Integer) (ValueUp :type Integer) (ValueDown :type Integer) (ValueMask :type Integer) (ValueItemId :type Integer) (ValueItemQuantity :type Integer) (ValueDelay :type "Float (single-precision)") (ValueSize :type "Float (single-precision)") (ValueDamage :type "Float (single-precision)") (ValueVariant :type Integer) (ValueSequence :type String))
  ;[1 0.5 0.5] (Server) Trigger Configure
  (set `self.TriggerName` NameSub)
  (set `self.TriggerValueTrigger` ValueTrigger)
  (set `self.TriggerValueUp` ValueUp)
  (set `self.TriggerValueDown` ValueDown)
  (`PersistenceComponent.SetDirty` (`self.ConanBuildingPersistence`) true 5.0))

(fn `InteractableActivateDisabled`
  (params (InteractingCharacter :type "ConanCharacter Object Reference"))
  (returns (ReturnValue :type Boolean))
  (return false))

(fn `InteractableGetUIModuleName`
  (returns (ReturnValue :type Name))
  (return "None"))

(fn `OnRep_TriggerName`)

(fn `OnRep_TriggerValueTrigger`)

(fn `PlaySound`
  (`GameplayStatics.PlaySoundAtLocation` "/Game/Sound/SFX/Weapons/Bow_Crossbow/sfx_crossbow_charge_click_Cue.sfx_crossbow_charge_click_Cue" (`self.K2_GetActorLocation` self) (struct) 1.0 1.0))

(fn `UserConstructionScript`
  (`parent.UserConstructionScript`))