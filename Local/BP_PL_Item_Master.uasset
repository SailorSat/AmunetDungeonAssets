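; BP_PL_Item_Master is a placeable item base in Conan Exiles that a player picks up by interacting with it.
; On activation it adds the source item template to the interacting ConanCharacter's shortcut bar or backpack, chosen by the AddToShortcutBar flag, then destroys itself.
; It supplies no interaction UI module and leaves loss of stability unhandled.
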(event `InteractableInterface.InteractableActivate`
  (params (Component :type "PrimitiveComponent Object Reference") (Instigator :type "PlayerController Object Reference") (HitIndex :type Integer) (TriggeredFromRadialWheel :type Boolean))
  (bind _sourceitemtemplateid (`self.SourceItemTemplateID`))
  (bind (_asconan_character _bsuccess) (cast `ConanCharacter` (`Controller.K2_GetPawn` Instigator) :!pure true))
  (if _bsuccess
    (if (`self.AddToShortcutBar`)
      (bind _returnvalue (`ConanCharacter.GetShortcutBarInventory` _asconan_character))
      (`ItemInventory.AddItemTemplate` _returnvalue _sourceitemtemplateid -1 1 true 1.0 -1.0)
      (else
        (bind _returnvalue_2 (`ConanCharacter.GetBackpackInventory` _asconan_character))
        (`ItemInventory.AddItemTemplate` _returnvalue_2 _sourceitemtemplateid -1 1 true 1.0 -1.0)))
    (`self.K2_DestroyActor` self)))

(event `self.StabilityLost`)

(fn `InteractableGetUIModuleName`
  (returns (ReturnValue :type Name))
  (return "None"))

(fn `UserConstructionScript`
  (`parent.UserConstructionScript`))