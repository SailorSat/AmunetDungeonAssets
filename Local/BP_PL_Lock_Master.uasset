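; Master lock placeable for Amunet Dungeon Assets that fires a named trigger when a player holds the required item.
; On interaction it checks backpack then shortcut bar, optionally consumes the item and calls ActivateTrigger on the server-cached ModController, or shows a need-key notification.
; Owners get a radial menu entry opening a config popup for trigger and item settings, which ConfigTrigger stores and marks dirty for persistence.
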(event `self.ReceiveBeginPlay`
  ;[1 0.5 0.5] (Server) BeginPlay
  (`parent.ReceiveBeginPlay`)
  (if (`KismetSystemLibrary.IsServer`)
    (bind _outactors (`GameplayStatics.GetAllActorsOfClass` "/Game/Mods/AmunetDungeonAssets/AmunetDungeonAssets_ModController.AmunetDungeonAssets_ModController_C"))
    (set `self.ModController` (`KismetArrayLibrary.Array_Get` _outactors))))

(event `InteractableInterface.InteractableActivate`
  (params (Component :type "PrimitiveComponent Object Reference") (Instigator :type "PlayerController Object Reference") (HitIndex :type Integer) (TriggeredFromRadialWheel :type Boolean))
  (bind _requireditemid (`self.RequiredItemID`))
  (bind _requireditemquantity (`self.RequiredItemQuantity`))
  (bind _removeitemafteruse (`self.RemoveItemAfterUse`))
  (bind _asconan_character (cast `ConanCharacter` (`Controller.K2_GetPawn` Instigator) :!pure true))
  ;[1 0.5 0.5] (Server) Interaction
  (bind _returnvalue (`ConanCharacter.GetBackpackInventory` _asconan_character))
  (bind _returnvalue_2 (`ConanCharacter.GetShortcutBarInventory` _asconan_character))
  (if (`ItemInventory.HasItemByTemplateID` _returnvalue _requireditemid _requireditemquantity)
    (if _removeitemafteruse
      (`ItemInventory.DeleteItemsByTemplate` _returnvalue _requireditemid _requireditemquantity))
    (`/Game/Mods/AmunetDungeonAssets/AmunetDungeonAssets_ModController.ActivateTrigger` (`self.ModController`) (`self.TriggerName`) (`self.TriggerValue`) Component Instigator HitIndex :!label _label)
    (elif (`ItemInventory.HasItemByTemplateID` _returnvalue_2 _requireditemid _requireditemquantity)
      (if _removeitemafteruse
        (`ItemInventory.DeleteItemsByTemplate` _returnvalue_2 _requireditemid _requireditemquantity)
        (goto _label)
        (else
          (goto _label)))
      (else
        (`ConanCharacter.ClientHUDShowNotification` _asconan_character (`self.NeedKeyText`) false)))))

(event `InteractableInterface.InteractableMenu`
  (params (RadialMenu :type "RadialMenu Object Reference") (HitIndex :type Integer))
  ;[0.5 1 1] (Client) Handle Menu Item
  (`parent.InteractableMenu` RadialMenu HitIndex)
  (if (`self.IsOwner` (`Controller.K2_GetPawn` (`UserWidget.GetOwningPlayer` RadialMenu)))
    (bind _returnvalue (`RadialMenu.AddItem` RadialMenu "ADA Config" (`/Game/Characters/SurvivalFunctionLibrary.GetBuildableObjectName` self) "/Game/UI/Textures/GUIs/Guild/T_EditButton.T_EditButton" "None" 0))
    (add `RadialMenuEntry.SignalClicked` _returnvalue (delegate `ClientClickedEdit`))))

(event `ClientClickedEdit`
  (params (menuEntry :type "RadialMenuEntry Object Reference"))
  ;[0.5 1 1] (Client) Handle Menu Item
  (`self.ClientLoadPopup`))

(event `ClientLoadPopup`
  ;[0.5 1 1] (Client) Trigger Configure
  (bind _returnvalue (`GUIModuleController.ActivateModule` (`GUIModuleController.GetGUIModuleController`) "TriggerConfig" true false))
  (bind _asw_ada_config_trigger (cast `/Game/Mods/AmunetDungeonAssets/UI/W_ADA_ConfigTrigger` _returnvalue))
  (`/Game/Mods/AmunetDungeonAssets/UI/W_ADA_ConfigTrigger.ConfigTrigger` _asw_ada_config_trigger self "" false (`self.TriggerName`) true (`self.TriggerValue`) true 0 false 0 false 0 false (`self.RequiredItemID`) true (`self.RequiredItemQuantity`) true 0.0 false 0.0 false 0.0 false 0 false))

(event `/Game/Mods/AmunetDungeonAssets/ADA_TriggerInterface.ConfigTrigger`
  (params (Name :type String) (NameSub :type String) (ValueTrigger :type Integer) (ValueUp :type Integer) (ValueDown :type Integer) (ValueMask :type Integer) (ValueItemId :type Integer) (ValueItemQuantity :type Integer) (ValueDelay :type "Float (single-precision)") (ValueSize :type "Float (single-precision)") (ValueDamage :type "Float (single-precision)") (ValueVariant :type Integer))
  ;[1 0.5 0.5] (Server) Trigger Configure
  (set `self.TriggerName` NameSub)
  (set `self.TriggerValue` ValueTrigger)
  (set `self.RequiredItemID` ValueItemId)
  (set `self.RequiredItemQuantity` ValueItemQuantity)
  (`PersistenceComponent.SetDirty` (`self.ConanBuildingPersistence`) true 5.0))

(fn `InteractableGetUIModuleName`
  (returns (ReturnValue :type Name))
  (return "None"))

(fn `UserConstructionScript`
  (`parent.UserConstructionScript`))