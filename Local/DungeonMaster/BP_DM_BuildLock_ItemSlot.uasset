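; Dungeon Master placeable item slot that acts as a lock, firing a named trigger based on whether it holds the required item ID.
; Inventory changes display the item's async-loaded static or skeletal mesh, offset by category, and the server sends the down or up value to the ADA ModController.
; Owners configure trigger name, values and item ID through a radial-menu popup, and edits mark building persistence dirty.
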(event `self.CleanUp`
  ;[0.62 0 0] Override and ignore cleanup as we need our slots for later.
)

(event `self.ReceiveBeginPlay`
  (bind _slot0static (`self.Slot0Static`))
  ;[1 1 1] BeginPlay
  (`parent.ReceiveBeginPlay`)
  (set `self.Initial Location Slot 0` (`SceneComponent.K2_GetComponentLocation` _slot0static))
  (set `self.Initial Rotation Slot 0` (`SceneComponent.K2_GetComponentRotation` _slot0static))
  (bind _returnvalue (`|GenericCreateObject` "/Script/ConanSandbox.ItemInventoryClientMonitor" self))
  (bind _output_get (set `self.ItemInventoryMonitor` _returnvalue))
  (`ItemInventoryClientMonitor.SetInventory` _output_get (`self.PlaceableInventory`))
  (`parent.ReceiveBeginPlay`)
  (if (`KismetSystemLibrary.IsServer`)
    (bind _outactors (`GameplayStatics.GetAllActorsOfClass` "/Game/Mods/AmunetDungeonAssets/AmunetDungeonAssets_ModController.AmunetDungeonAssets_ModController_C"))
    (set `self.ModController` (`KismetArrayLibrary.Array_Get` _outactors))))

(event `TriggerOthers`
  (params (IsValid :type Boolean))
  ;[1 1 1] Trigger Others
  (if (`KismetSystemLibrary.IsServer`)
    (`/Game/Mods/AmunetDungeonAssets/AmunetDungeonAssets_ModController.ActivateTrigger` (`self.ModController`) (`self.TriggerName`) (select `bool` IsValid :`false` (`self.TriggerValueUp`) :`true` (`self.TriggerValueDown`)) (`self.SavedComponent`) (`self.InteractingInstigator`) (`self.SavedHitIndex`))))

(event `InteractableInterface.InteractableActivate`
  (params (Component :type "PrimitiveComponent Object Reference") (Instigator :type "PlayerController Object Reference") (HitIndex :type Integer) (TriggeredFromRadialWheel :type Boolean))
  ;[1 1 1] Save Component and HitIndex
  (bind _output_get (set `self.SavedComponent` Component))
  (bind _output_get_2 (set `self.InteractingInstigator` Instigator))
  (bind _output_get_3 (set `self.SavedHitIndex` HitIndex))
  (`InteractableInterface.InteractableActivate` (`self.BP_BAC_Storage`) _output_get _output_get_2 _output_get_3 TriggeredFromRadialWheel))

(event `self.PlaceableInventory.SignalItemRemoved`
  (params (index :type Integer) (item :type "GameItem Object Reference") (dstInventory :type "ItemInventory Object Reference") (dstIndex :type Integer))
  (bind _locationmod (`self.LocationMod`))
  (bind _slot0skeletal (`self.Slot0Skeletal`))
  (bind _placeableinventory (`self.PlaceableInventory`))
  (bind _slot0static (`self.Slot0Static`))
  (bind _initial_location_slot_0 (`self.Initial Location Slot 0`))
  (bind _initial_rotation_slot_0 (`self.Initial Rotation Slot 0`))
  (bind _rotationmod (`self.RotationMod`))
  (bind _returnvalue (`ItemInventory.GetItem` _placeableinventory 0))
  (bind _returnvalue_2 (`KismetSystemLibrary.IsValid` (`ItemInventory.GetItem` _placeableinventory 0)))
  ;[1 1 1] Handle Item Changes
  (`StaticMeshComponent.SetStaticMesh` _slot0static (`self.EmptyStaticMesh`) :!label _label)
  (`SkinnedMeshComponent.SetSkinnedAssetAndUpdate` _slot0skeletal (`self.EmptySkeletalMesh`) true)
  (if _returnvalue_2
    (`self.CheckForValidItems` 0)
    (`self.TriggerOthers` (`self.IsRequiredItem`))
    (bind _object (`|LoadAsset` (`GameItem.GetVisualStaticMesh` _returnvalue)))
    (`/Engine/EditorBlueprintResources/StandardMacros.IsValid` _object
      (:`Is Valid`
        (`SceneComponent.K2_SetWorldLocationAndRotation` _slot0static _initial_location_slot_0 _initial_rotation_slot_0 false false)
        (`SceneComponent.ResetRelativeTransform` _slot0static)
        (`StaticMeshComponent.SetStaticMesh` _slot0static _object)
        (`SceneComponent.K2_AddRelativeLocation` _slot0static _locationmod false false)
        (`SceneComponent.K2_AddRelativeRotation` _slot0static _rotationmod false false)
        (`SceneComponent.SetRelativeScale3D` _slot0static (1.0 1.0 1.0)))
      (:`Is Not Valid`
        (bind _object_2 (`|LoadAsset` (`GameItem.GetVisualSkeletalMesh` _returnvalue)))
        (`/Engine/EditorBlueprintResources/StandardMacros.IsValid` _object_2
          (:`Is Valid`
            (`SceneComponent.K2_SetWorldLocationAndRotation` _slot0skeletal _initial_location_slot_0 _initial_rotation_slot_0 false false)
            (`SceneComponent.ResetRelativeTransform` _slot0skeletal)
            (`SkinnedMeshComponent.SetSkinnedAssetAndUpdate` _slot0skeletal _object_2 true)
            (`SceneComponent.K2_AddRelativeLocation` _slot0skeletal _locationmod false false)
            (`SceneComponent.K2_AddRelativeRotation` _slot0skeletal _rotationmod false false)
            (`SceneComponent.SetRelativeScale3D` _slot0skeletal (1.0 1.0 1.0))))))
    (else
      (`self.TriggerOthers` _returnvalue_2))))

(event `self.PlaceableInventory.SignalItemAdded`
  (params (index :type Integer) (item :type "GameItem Object Reference") (srcInventory :type "ItemInventory Object Reference") (srcIndex :type Integer))
  ;[1 1 1] Handle Item Changes
  (goto _label))

(event `self.PlaceableInventory.SignalItemFloatStatChanged`
  (params (item :type "GameItem Object Reference") (statID :type "EItemFloatStatID Enum" :default "WeaponStaminaHeavyChargedRegenModifier") (statValue :type "Float (single-precision)") (deltaValue :type "Float (single-precision)"))
  ;[1 1 1] Handle Item Changes
  (goto _label))

(event `self.PlaceableInventory.SignalItemIntStatChanged`
  (params (item :type "GameItem Object Reference") (statID :type "EItemIntStatID Enum" :default "MaxStackSize") (statValue :type Integer) (deltaValue :type Integer))
  ;[1 1 1] Handle Item Changes
  (goto _label))

(event `InteractableInterface.InteractableMenu`
  (params (RadialMenu :type "RadialMenu Object Reference") (HitIndex :type Integer))
  ;[0.5 1 1] (Client) Handle Menu Item
  (`parent.InteractableMenu` RadialMenu HitIndex)
  (if (`self.IsOwner` (`Controller.K2_GetPawn` (`UserWidget.GetOwningPlayer` RadialMenu)))
    (bind _returnvalue (`RadialMenu.AddItem` RadialMenu "ADA Config" (`/Game/Characters/SurvivalFunctionLibrary.GetBuildableObjectName` self) "/Game/UI/Textures/GUIs/Guild/T_EditButton.T_EditButton" "None" 0))
    (add `RadialMenuEntry.SignalClicked` _returnvalue (delegate `ClientClickedEdit`))))

(event `ClientClickedEdit`
  (params (menuEntry :type "RadialMenuEntry Object Reference"))
  ;[0.5 1 1] (Client) Handle Menu Item
  (`self.ClientLoadPopup`))

(event `ClientLoadPopup`
  ;[0.5 1 1] (Client) Trigger Configure
  (bind _returnvalue (`GUIModuleController.ActivateModule` (`GUIModuleController.GetGUIModuleController`) "TriggerConfig" true false))
  (bind _asw_ada_config_trigger (cast `/Game/Mods/AmunetDungeonAssets/UI/W_ADA_ConfigTrigger` _returnvalue))
  (`/Game/Mods/AmunetDungeonAssets/UI/W_ADA_ConfigTrigger.ConfigTrigger` _asw_ada_config_trigger self "" false (`self.TriggerName`) true 0 false (`self.TriggerValueUp`) true (`self.TriggerValueDown`) true 0 false (`self.RequiredItemID`) true 0 false 0.0 false 0.0 false 0.0 false 0 false "" false))

(event `/Game/Mods/AmunetDungeonAssets/ADA_TriggerInterface.ConfigTrigger`
  (params (Name :type String) (NameSub :type String) (ValueTrigger :type Integer) (ValueUp :type Integer) (ValueDown :type Integer) (ValueMask :type Integer) (ValueItemId :type Integer) (ValueItemQuantity :type Integer) (ValueDelay :type "Float (single-precision)") (ValueSize :type "Float (single-precision)") (ValueDamage :type "Float (single-precision)") (ValueVariant :type Integer) (ValueSequence :type String))
  ;[1 0.5 0.5] (Server) Trigger Configure
  (set `self.TriggerName` NameSub)
  (set `self.TriggerValueUp` ValueUp)
  (set `self.TriggerValueDown` ValueDown)
  (set `self.RequiredItemID` ValueItemId)
  (`PersistenceComponent.SetDirty` (`self.ConanBuildingPersistence`) true 5.0))

(fn `CheckForValidItems`
  (params (index :type Integer))
  (bind _returnvalue (`ItemInventory.GetItem` (`self.PlaceableInventory`) index))
  (set `self.IsRequiredItem` (== (`GameItem.TemplateID` _returnvalue) (`self.RequiredItemID`)))
  (if (`|EnumEquality` (`GameItem.GetGUICategory` _returnvalue) "BuildingItem")
    (set `self.LocationMod` (0.0 0.0 0.0))
    (set `self.RotationMod` (struct))
    (else
      (set `self.LocationMod` (0.0 0.0 3.0))
      (set `self.RotationMod` (struct :`Roll` 90.0)))))

(fn `InteractableGetUIModuleName`
  (returns (ReturnValue :type Name))
  (return "None"))

(fn `UserConstructionScript`
  (`parent.UserConstructionScript`))