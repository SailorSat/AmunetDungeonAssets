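; Breakable green curtain wall decoration for the DungeonMaster set that tears when damaged and can be repaired by its owner.
; On the server, point damage sets IsBroken and an owner's interaction clears it; other interactions pass to the parent.
; The IsBroken RepNotify drives SetBrokenState, which swaps intact and torn meshes with a sound.
; BeginPlay also applies the current state, so that sound plays on spawn.
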(event `self.ReceiveBeginPlay`
  ;[1 1 0.5] (Both) BeginPlay
  (`self.SetBrokenState` (`self.IsBroken`))
  (`parent.ReceiveBeginPlay`))

(event `self.ReceivePointDamage`
  (params (Damage :type "Float (single-precision)") (DamageType :type "DamageType Object Reference") (HitLocation :type "Vector Structure") (HitNormal :type "Vector Structure") (HitComponent :type "PrimitiveComponent Object Reference") (BoneName :type Name) (ShotFromDirection :type "Vector Structure") (InstigatedBy :type "Controller Object Reference") (DamageCauser :type "Actor Object Reference") (HitInfo :type "HitResult Structure (by ref)"))
  ;[1 0.5 0.5] (Server) PointDamage
  (`parent.ReceivePointDamage` Damage DamageType HitLocation HitNormal HitComponent BoneName ShotFromDirection InstigatedBy DamageCauser HitInfo)
  (if (not (`self.IsBroken`))
    (set `self.IsBroken` true)))

(event `InteractableInterface.InteractableActivate`
  (params (Component :type "PrimitiveComponent Object Reference") (Instigator :type "PlayerController Object Reference") (HitIndex :type Integer) (TriggeredFromRadialWheel :type Boolean))
  ;[1 0.5 0.5] (Server) OnActivate
  (if (`self.IsOwner` (`Controller.K2_GetPawn` Instigator) true)
    (if (`self.IsBroken`)
      (set `self.IsBroken` false)
      (else
        (`parent.InteractableActivate` Component Instigator HitIndex false :!label _label)))
    (else
      (goto _label))))

(event `OnBreak`
  ;[1 1 0.5] (Both) Sound
  (`GameplayStatics.PlaySoundAtLocation` "/Game/Sound/SFX/Impacts/Impact_Tails/Leather/sfx_foley_tail_leather_thin_2.sfx_foley_tail_leather_thin_2" (`self.K2_GetActorLocation` self) (struct) 1.0 1.0)
  (`StaticMeshComponent.SetStaticMesh` (`self.StaticMesh`) "/Game/Mods/AmunetDungeonAssets/DungeonMaster/Meshes/WallDeco/SM_DM_WallDeco_Curtain_GreenTorn.SM_DM_WallDeco_Curtain_GreenTorn"))

(event `OnRepair`
  ;[1 1 0.5] (Both) Sound
  (`GameplayStatics.PlaySoundAtLocation` "/Game/Sound/SFX/Impacts/Shield/sfx_blunt_shield_hit_block_wood_Cue.sfx_blunt_shield_hit_block_wood_Cue" (`self.K2_GetActorLocation` self) (struct) 1.0 1.0)
  (`StaticMeshComponent.SetStaticMesh` (`self.StaticMesh`) "/Game/Mods/AmunetDungeonAssets/DungeonMaster/Meshes/WallDeco/SM_DM_WallDeco_Curtain_Green.SM_DM_WallDeco_Curtain_Green"))

(fn `OnRep_IsBroken`
  (`self.SetBrokenState` (`self.IsBroken`)))

(fn `SetBrokenState`
  (params (NewState :type Boolean))
  (if NewState
    (`self.OnBreak`)
    (else
      (`self.OnRepair`))))

(fn `UserConstructionScript`
  (`parent.UserConstructionScript`))