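; Dungeon Master magic hatch, a configurable trigger object that acts as a curse-wall barrier in one of four colors.
; Open and close events from the parent hide or show the mesh and switch its Pawn collision between overlap and block.
; A variant set through the server trigger config selects the material on BeginPlay and OnRep.
; The client popup exposes that variant in the TriggerConfig UI module.
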(event `self.ReceiveBeginPlay`
  ;[1 1 1] Add Variant
  (`parent.ReceiveBeginPlay`)
  (`self.SetVariant` (`self.DynamicVariant`)))

(event `/Game/Systems/Building/Placeables/BP_PL_Hatch.ClosedToOpenNormal`
  (bind _staticmesh (`self.StaticMesh`))
  ;[1 1 1] Animation
  (`SceneComponent.SetVisibility` _staticmesh false false :!label _label)
  (`PrimitiveComponent.SetCollisionResponseToChannel` _staticmesh "ECC_Pawn" "ECR_Overlap"))

(event `/Game/Systems/Building/Placeables/BP_PL_Hatch.ClosedToOpenReverse`
  ;[1 1 1] Animation
  (goto _label))

(event `/Game/Systems/Building/Placeables/BP_PL_Hatch.OpenNormalToClosed`
  (bind _staticmesh (`self.StaticMesh`))
  ;[1 1 1] Animation
  (`SceneComponent.SetVisibility` _staticmesh true false :!label _label_2)
  (`PrimitiveComponent.SetCollisionResponseToChannel` _staticmesh "ECC_Pawn" "ECR_Block"))

(event `/Game/Systems/Building/Placeables/BP_PL_Hatch.OpenReversedToClosed`
  ;[1 1 1] Animation
  (goto _label_2))

(event `/Game/Mods/AmunetDungeonAssets/ADA_TriggerInterface.ConfigTrigger`
  (params (Name :type String) (NameSub :type String) (ValueTrigger :type Integer) (ValueUp :type Integer) (ValueDown :type Integer) (ValueMask :type Integer) (ValueItemId :type Integer) (ValueItemQuantity :type Integer) (ValueDelay :type "Float (single-precision)") (ValueSize :type "Float (single-precision)") (ValueDamage :type "Float (single-precision)") (ValueVariant :type Integer) (ValueSequence :type String))
  ;[1 0.5 0.5] (Server) Trigger Configure
  (bind _output_get (set `self.DynamicVariant` ValueVariant))
  (`parent.ConfigTrigger` Name NameSub ValueTrigger ValueUp ValueDown ValueMask ValueItemId ValueItemQuantity ValueDelay ValueSize ValueDamage _output_get ""))

(event `self.ClientLoadPopup`
  ;[0.5 1 1] (Client) Trigger Configure
  (bind _returnvalue (`GUIModuleController.ActivateModule` (`GUIModuleController.GetGUIModuleController`) "TriggerConfig" true false))
  (bind _asw_ada_config_trigger (cast `/Game/Mods/AmunetDungeonAssets/UI/W_ADA_ConfigTrigger` _returnvalue))
  (`/Game/Mods/AmunetDungeonAssets/UI/W_ADA_ConfigTrigger.ConfigTrigger` _asw_ada_config_trigger self (`self.TriggerName`) true "" false 0 false 0 false 0 false 0 false 0 false 0 false 0.0 false 0.0 false 0.0 false (`self.DynamicVariant`) true "" false))

(fn `OnRep_DynamicVariant`
  (`self.SetVariant` (`self.DynamicVariant`)))

(fn `SetVariant`
  (params (Variant :type Integer))
  (bind _staticmesh (`self.StaticMesh`))
  (switch `int` Variant
    (:`Default`
      (`PrimitiveComponent.SetMaterial` _staticmesh 0 "/Game/Mods/AmunetDungeonAssets/Dummy/Materials/ADA_CurseWall_Yellow.ADA_CurseWall_Yellow"))
    (:`1`
      (`PrimitiveComponent.SetMaterial` _staticmesh 0 "/Game/Mods/AmunetDungeonAssets/Dummy/Materials/ADA_CurseWall_Blue.ADA_CurseWall_Blue"))
    (:`2`
      (`PrimitiveComponent.SetMaterial` _staticmesh 0 "/Game/Mods/AmunetDungeonAssets/Dummy/Materials/ADA_CurseWall_Green.ADA_CurseWall_Green"))
    (:`3`
      (`PrimitiveComponent.SetMaterial` _staticmesh 0 "/Game/Mods/AmunetDungeonAssets/Dummy/Materials/ADA_CurseWall_Red.ADA_CurseWall_Red"))))

(fn `UserConstructionScript`
  (`parent.UserConstructionScript`))