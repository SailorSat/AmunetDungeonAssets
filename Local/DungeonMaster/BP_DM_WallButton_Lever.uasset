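; Wall lever for the DungeonMaster module that toggles between up and down and fires a named trigger on the ModController.
; On server activation it flips the replicated IsSet, ignoring input while the last animation runs, and sends the up or down trigger value.
; OnRep and BeginPlay apply the state through SetLeverState, which plays a sound and runs one timeline forward or in reverse to rotate the mesh.
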(event `self.ReceiveBeginPlay`
  ;[1 1 0.5] (Both) BeginPlay
  (`parent.ReceiveBeginPlay`)
  (`self.SetLeverState` (`self.IsSet`)))

(event `UpToDown`
  ;[1 1 0.5] (Both) Animation and Sound
  (`self.PlaySound`)
  (bind (_direction _alpha) (`Timeline|Timeline_UpToDown` :!via `PlayFromStart` :!label _label)
    (:`Update`
      (`SceneComponent.K2_SetRelativeRotation` (`self.StaticMesh`) (`KismetMathLibrary.MakeRotator` _alpha 0.0 90.0) false false))
    (:`Finished`
      (set `self.IsLastAnimationFinished` true))))

(event `DownToUp`
  ;[1 1 0.5] (Both) Animation and Sound
  (`self.PlaySound`)
  (goto _label :!via `ReverseFromEnd`))

(event `InteractableInterface.InteractableActivate`
  (params (Component :type "PrimitiveComponent Object Reference") (Instigator :type "PlayerController Object Reference") (HitIndex :type Integer))
  (bind _isset (`self.IsSet`))
  ;[1 0.5 0.5] (Server) Interactable Activate
  (if (`self.IsLastAnimationFinished`)
    (set `self.IsLastAnimationFinished` false)
    (if _isset
      (set `self.IsSet` false)
      (else
        (set `self.IsSet` true)))
    (`/Game/Mods/AmunetDungeonAssets/AmunetDungeonAssets_ModController.ActivateTrigger` (`self.ModController`) (`self.TriggerName`) (select `bool` _isset :`false` (`self.TriggerValueUp`) :`true` (`self.TriggerValueDown`)) Component Instigator HitIndex)))

(fn `OnRep_IsSet`
  (`self.SetLeverState` (`self.IsSet`)))

(fn `SetLeverState`
  (params (NewState :type Boolean))
  (if NewState
    (`self.UpToDown`)
    (else
      (`self.DownToUp`))))

(fn `UserConstructionScript`
  (`parent.UserConstructionScript`))