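; Dungeon Master wall decoration receptor: a placeable that plays a hit sound on point damage and fires a named trigger.
; If a player controller caused the damage, it passes its trigger name and value to the ADA ModController found on server BeginPlay.
; Owners get an "ADA Config" radial menu entry opening the TriggerConfig popup.
; ConfigTrigger stores the edited name and value and marks building persistence dirty.
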(event `self.ReceiveBeginPlay`
  ;[1 0.5 0.5] (Server) BeginPlay
  (`parent.ReceiveBeginPlay`)
  (if (`KismetSystemLibrary.IsServer`)
    (bind _outactors (`GameplayStatics.GetAllActorsOfClass` "/Game/Mods/AmunetDungeonAssets/AmunetDungeonAssets_ModController.AmunetDungeonAssets_ModController_C"))
    (set `self.ModController` (`KismetArrayLibrary.Array_Get` _outactors))))

(event `InteractableInterface.InteractableMenu`
  (params (RadialMenu :type "RadialMenu Object Reference") (HitIndex :type Integer))
  ;[0.5 1 1] (Client) Handle Menu Item
  (`parent.InteractableMenu` RadialMenu HitIndex)
  (if (`self.IsOwner` (`Controller.K2_GetPawn` (`UserWidget.GetOwningPlayer` RadialMenu)))
    (bind _returnvalue (`RadialMenu.AddItem` RadialMenu "ADA Config" (`/Game/Characters/SurvivalFunctionLibrary.GetBuildableObjectName` self) "/Game/UI/Textures/GUIs/Guild/T_EditButton.T_EditButton" "None" 0))
    (add `RadialMenuEntry.SignalClicked` _returnvalue (delegate `ClientClickedEdit`))))

(event `self.ReceivePointDamage`
  (params (Damage :type "Float (single-precision)") (DamageType :type "DamageType Object Reference") (HitLocation :type "Vector Structure") (HitNormal :type "Vector Structure") (HitComponent :type "PrimitiveComponent Object Reference") (BoneName :type Name) (ShotFromDirection :type "Vector Structure") (InstigatedBy :type "Controller Object Reference") (DamageCauser :type "Actor Object Reference") (HitInfo :type "HitResult Structure (by ref)"))
  ;[1 0.5 0.5] (Server) PointDamage
  (`self.OnActivate`)
  (bind _asplayer_controller (cast `PlayerController` InstigatedBy)
    (:`then`
      (`/Game/Mods/AmunetDungeonAssets/AmunetDungeonAssets_ModController.ActivateTrigger` (`self.ModController`) (`self.TriggerName`) (`self.TriggerValue`) HitComponent _asplayer_controller 0))
    (:`CastFailed`
      _))
  (`parent.ReceivePointDamage` Damage DamageType HitLocation HitNormal HitComponent BoneName ShotFromDirection InstigatedBy DamageCauser HitInfo))

(event `ClientClickedEdit`
  (params (menuEntry :type "RadialMenuEntry Object Reference"))
  ;[0.5 1 1] (Client) Handle Menu Item
  (`self.ClientLoadPopup`))

(event `ClientLoadPopup`
  ;[0.5 1 1] (Client) Trigger Configure
  (bind _returnvalue (`GUIModuleController.ActivateModule` (`GUIModuleController.GetGUIModuleController`) "TriggerConfig" true false))
  (bind _asw_ada_config_trigger (cast `/Game/Mods/AmunetDungeonAssets/UI/W_ADA_ConfigTrigger` _returnvalue))
  (`/Game/Mods/AmunetDungeonAssets/UI/W_ADA_ConfigTrigger.ConfigTrigger` _asw_ada_config_trigger self (`self.TriggerName`) false "" false (`self.TriggerValue`) true 0 false 1 false 0 false 0 false 0 false 0.0 false 0.0 false 0.0 false 0 false))

(event `/Game/Mods/AmunetDungeonAssets/ADA_TriggerInterface.ConfigTrigger`
  (params (Name :type String) (NameSub :type String) (ValueTrigger :type Integer) (ValueUp :type Integer) (ValueDown :type Integer) (ValueMask :type Integer) (ValueItemId :type Integer) (ValueItemQuantity :type Integer) (ValueDelay :type "Float (single-precision)") (ValueSize :type "Float (single-precision)") (ValueDamage :type "Float (single-precision)") (ValueVariant :type Integer))
  ;[1 0.5 0.5] (Server) Trigger Configure
  (set `self.TriggerName` Name)
  (set `self.TriggerValue` ValueTrigger)
  (`PersistenceComponent.SetDirty` (`self.ConanBuildingPersistence`) true 5.0))

(event `OnActivate`
  ;[1 1 0.5] (Both) Sound
  (`GameplayStatics.PlaySoundAtLocation` "/Game/Sound/SFX/Impacts/Arrows/Special/sfx_arrow_hit_mechanic_wet_Cue.sfx_arrow_hit_mechanic_wet_Cue" (`self.K2_GetActorLocation` self) (struct) 1.0 1.0))

(fn `UserConstructionScript`
  (`parent.UserConstructionScript`))