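; Buildable Dungeon Master magic bridge trap whose mesh shows while something overlaps its trigger box and hides when the box empties.
; The server toggles IsDown on overlap, and a rep-notify passes it through SetTrapState to fire/reset events that change only visibility, not collision.
; Owners pick one of four curse-wall color materials through a radial-menu config popup; DynamicVariant is applied via rep-notify and marked dirty for persistence.
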(event `self.ReceiveBeginPlay`
  ;[1 1 0.5] (Both) BeginPlay
  (`parent.ReceiveBeginPlay`)
  (`self.SetTrapState` (`self.IsDown`))
  (`self.SetVariant` (`self.DynamicVariant`)))

(event `MulticastTrapReset`
  ;[1 1 0.5] (Both) Animation and Sound
  (`SceneComponent.SetVisibility` (`self.StaticMesh`) false false))

(event `MulticastTrapFire`
  ;[1 1 0.5] (Both) Animation and Sound
  (`SceneComponent.SetVisibility` (`self.StaticMesh`) true false))

(event `self.TrapTriggerBox.OnComponentBeginOverlap`
  (params (OverlappedComponent :type "PrimitiveComponent Object Reference") (OtherActor :type "Actor Object Reference") (OtherComp :type "PrimitiveComponent Object Reference") (OtherBodyIndex :type Integer) (bFromSweep :type Boolean) (SweepResult :type "HitResult Structure (by ref)"))
  ;[1 0.5 0.5] (Server) OnOverlap
  (if (`KismetSystemLibrary.IsServer`)
    (if (`self.IsDown`)
      _
      (elif (not (== (`KismetArrayLibrary.Array_Length` (`PrimitiveComponent.GetOverlappingActors` (`self.TrapTriggerBox`) null)) 0))
        (set `self.IsDown` true)))))

(event `self.TrapTriggerBox.OnComponentEndOverlap`
  (params (OverlappedComponent :type "PrimitiveComponent Object Reference") (OtherActor :type "Actor Object Reference") (OtherComp :type "PrimitiveComponent Object Reference") (OtherBodyIndex :type Integer))
  ;[1 0.5 0.5] (Server) OnOverlap
  (if (`KismetSystemLibrary.IsServer`)
    (if (`self.IsDown`)
      (if (== (`KismetArrayLibrary.Array_Length` (`PrimitiveComponent.GetOverlappingActors` (`self.TrapTriggerBox`) null)) 0)
        (set `self.IsDown` false)))))

(event `InteractableInterface.InteractableMenu`
  (params (RadialMenu :type "RadialMenu Object Reference") (HitIndex :type Integer))
  ;[0.5 1 1] (Client) Handle Menu Item
  (`parent.InteractableMenu` RadialMenu HitIndex)
  (if (`self.IsOwner` (`Controller.K2_GetPawn` (`UserWidget.GetOwningPlayer` RadialMenu)))
    (bind _returnvalue (`RadialMenu.AddItem` RadialMenu "ADA Config" (`/Game/Characters/SurvivalFunctionLibrary.GetBuildableObjectName` self) "/Game/Mods/AmunetDungeonAssets/UI/T_icon_edit.T_icon_edit" "None" 0))
    (add `RadialMenuEntry.SignalClicked` _returnvalue (delegate `ClientClickedEdit`))))

(event `ClientClickedEdit`
  (params (menuEntry :type "RadialMenuEntry Object Reference"))
  ;[0.5 1 1] (Client) Handle Menu Item
  (`self.ClientLoadPopup`))

(event `ClientLoadPopup`
  ;[0.5 1 1] (Client) Trigger Configure
  (bind _returnvalue (`GUIModuleController.ActivateModule` (`GUIModuleController.GetGUIModuleController`) "TriggerConfig" true false))
  (bind _asw_ada_config_trigger (cast `/Game/Mods/AmunetDungeonAssets/UI/W_ADA_ConfigTrigger` _returnvalue))
  (`/Game/Mods/AmunetDungeonAssets/UI/W_ADA_ConfigTrigger.ConfigTrigger` _asw_ada_config_trigger self "" false "" false 0 false 0 false 0 false 0 false 0 false 0 false 0.0 false 0.0 false 0.0 false (`self.DynamicVariant`) true "" false))

(event `/Game/Mods/AmunetDungeonAssets/ADA_TriggerInterface.ConfigTrigger`
  (params (Name :type String) (NameSub :type String) (ValueTrigger :type Integer) (ValueUp :type Integer) (ValueDown :type Integer) (ValueMask :type Integer) (ValueItemId :type Integer) (ValueItemQuantity :type Integer) (ValueDelay :type "Float (single-precision)") (ValueSize :type "Float (single-precision)") (ValueDamage :type "Float (single-precision)") (ValueVariant :type Integer) (ValueSequence :type String))
  ;[1 0.5 0.5] (Server) Trigger Configure
  (set `self.DynamicVariant` ValueVariant)
  (`PersistenceComponent.SetDirty` (`self.ConanBuildingPersistence`) true 5.0))

(fn `CanBePlaced`
  (params (AttachTo :type "BuildableBase Object Reference") (InstanceIndex :type Integer))
  (returns (FailedMessage :type String) (ReturnValue :type "ECanBePlacedResult Enum"))
  (bind (_failedmessage _returnvalue) (`parent.CanBePlaced` AttachTo InstanceIndex))
  (return _failedmessage _returnvalue))

(fn `InteractableGetUIModuleName`
  (returns (ReturnValue :type Name))
  (return "None"))

(fn `OnRep_DynamicVariant`
  (`self.SetVariant` (`self.DynamicVariant`)))

(fn `OnRep_IsSet`
  (`self.SetTrapState` (`self.IsDown`)))

(fn `SetTrapState`
  (params (NewState :type Boolean))
  (if NewState
    (`self.MulticastTrapFire`)
    (else
      (`self.MulticastTrapReset`))))

(fn `SetVariant`
  (params (Variant :type Integer))
  (bind _staticmesh (`self.StaticMesh`))
  (switch `int` Variant
    (:`Default`
      (`PrimitiveComponent.SetMaterial` _staticmesh 0 "/Game/Mods/AmunetDungeonAssets/Dummy/Materials/ADA_CurseWall_Yellow.ADA_CurseWall_Yellow"))
    (:`1`
      (`PrimitiveComponent.SetMaterial` _staticmesh 0 "/Game/Mods/AmunetDungeonAssets/Dummy/Materials/ADA_CurseWall_Blue.ADA_CurseWall_Blue"))
    (:`2`
      (`PrimitiveComponent.SetMaterial` _staticmesh 0 "/Game/Mods/AmunetDungeonAssets/Dummy/Materials/ADA_CurseWall_Green.ADA_CurseWall_Green"))
    (:`3`
      (`PrimitiveComponent.SetMaterial` _staticmesh 0 "/Game/Mods/AmunetDungeonAssets/Dummy/Materials/ADA_CurseWall_Red.ADA_CurseWall_Red"))))

(fn `UserConstructionScript`
  (`parent.UserConstructionScript`))