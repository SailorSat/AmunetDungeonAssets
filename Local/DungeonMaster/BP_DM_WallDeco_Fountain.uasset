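; Interactable dungeon fountain decoration that a player can drink from.
; On activation it plays a swallow sound, then calls ServerDrink on the pawn's hunger component.
; If the pawn also has a buff system, it adds a heavy chilling effect buff and records a DrinkFromWell journey event on the server through the player character interface.
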(event `InteractableInterface.InteractableActivate`
  (params (Component :type "PrimitiveComponent Object Reference") (Instigator :type "PlayerController Object Reference") (HitIndex :type Integer) (TriggeredFromRadialWheel :type Boolean))
  (bind _returnvalue (`Controller.K2_GetPawn` Instigator))
  (bind _returnvalue_2 (`self.K2_GetComponentsByClass` _returnvalue "/Game/Systems/Hunger/BP_HungerSystem.BP_HungerSystem_C"))
  (bind _returnvalue_3 (`self.K2_GetComponentsByClass` _returnvalue "/Game/Systems/Buffs/00_BP_AC_BuffSystem.00_BP_AC_BuffSystem_C"))
  (`GameplayStatics.PlaySoundAtLocation` "/Game/Sound/Voiceover/Male_emotes/Male_1/Body_Feedback/vocal_male_drink_swallow_Cue.vocal_male_drink_swallow_Cue" (`self.K2_GetActorLocation` Instigator))
  (if (> (`KismetArrayLibrary.Array_Length` _returnvalue_2) 0)
    (`/Game/Systems/Hunger/BP_HungerSystem.ServerDrink` (`KismetArrayLibrary.Array_Get` _returnvalue_2) 100.0)
    (if (> (`KismetArrayLibrary.Array_Length` _returnvalue_3) 0)
      (`/Game/Systems/Buffs/00_BP_AC_BuffSystem.AddBuff` (`KismetArrayLibrary.Array_Get` _returnvalue_3) "/Game/Systems/Buffs/TemperatureBuffs/BP_AC_Buff_ChillingEffect_Heavy.BP_AC_Buff_ChillingEffect_Heavy_C" 0 null)
      (`self.Update Journey Event` Instigator))))

(fn `Update Journey Event`
  (params (Instigator :type "PlayerController Object Reference"))
  (if (`KismetSystemLibrary.IsServer`)
    (bind _asbase_player_char_interface (cast `/Game/Systems/Interfaces/BasePlayerCharInterface` (`Controller.K2_GetPawn` Instigator)))
    (`/Game/Systems/Interfaces/BasePlayerCharInterface.AddJourneyEventInterfaceCall` _asbase_player_char_interface "DrinkFromWell")))

(fn `UserConstructionScript`
  (`parent.UserConstructionScript`))