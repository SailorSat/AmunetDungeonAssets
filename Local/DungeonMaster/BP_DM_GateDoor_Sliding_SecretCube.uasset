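; BP_DM_GateDoor_Sliding_SecretCube is a sliding gate door variant that kills whatever stands in its KillBox when it closes.
; Both closing events, from normal-open and reversed-open, apply massive health-type damage to every overlapping actor, then call the parent logic.
; The damage is a single overlap query taken as the close event fires, not a continuous check during movement.
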(event `self.OpenReversedToClosed`
  (for _array_element (`PrimitiveComponent.GetOverlappingActors` (`self.KillBox`) null)
    (`GameplayStatics.ApplyDamage` _array_element 50000000.0 null self "/Game/Systems/Progression/DmgTypeHealth_BP.DmgTypeHealth_BP_C"))
  (`parent.OpenReversedToClosed`))

(event `self.OpenNormalToClosed`
  (for _array_element (`PrimitiveComponent.GetOverlappingActors` (`self.KillBox`) null)
    (`GameplayStatics.ApplyDamage` _array_element 50000000.0 null self "/Game/Systems/Progression/DmgTypeHealth_BP.DmgTypeHealth_BP_C"))
  (`parent.OpenNormalToClosed`))

(fn `UserConstructionScript`
  (`parent.UserConstructionScript`))