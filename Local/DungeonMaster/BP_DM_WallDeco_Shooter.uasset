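; Dungeon Master wall decoration trap that fires crossbow projectiles from two side boxes when interacted with or triggered.
; On the server it registers by trigger name with the Amunet Dungeon Assets mod controller, and a timeline times the shots, each with slight random pitch and yaw.
; An owner-only radial menu entry opens a popup to configure trigger name and damage, and the server marks those edits for persistence.
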(event `self.ReceiveBeginPlay`
  ;[1 1 0.5] (Both) BeginPlay
  (`parent.ReceiveBeginPlay`)
  (`self.SetDamage` (`self.DynamicDamage`))
  (set `self.InitialLocationLeft` (`SceneComponent.K2_GetComponentLocation` (`self.BoxLeft`)))
  (set `self.InitialLocationRight` (`SceneComponent.K2_GetComponentLocation` (`self.BoxRight`)))
  (set `self.InitialRotation` (`self.K2_GetActorRotation` self))
  (if (`KismetSystemLibrary.IsServer`)
    (bind _outactors (`GameplayStatics.GetAllActorsOfClass` "/Game/Mods/AmunetDungeonAssets/AmunetDungeonAssets_ModController.AmunetDungeonAssets_ModController_C"))
    (bind _output_get (set `self.ModController` (`KismetArrayLibrary.Array_Get` _outactors)))
    (`/Game/ModsShared/AmunetDungeonAssets/Interfaces/ADA_I_TriggerController.RegisterTriggerTarget` _output_get self (`self.TriggerName`))))

(event `self.ReceiveEndPlay`
  (params (EndPlayReason :type "EEndPlayReason Enum" :default "Destroyed"))
  ;[1 1 0.5] (Both) BeginPlay
  (`parent.ReceiveEndPlay` EndPlayReason)
  (`/Game/Systems/BP_MacroGlobal.IsValid+Branch` (`self.ModController`) (`KismetSystemLibrary.IsServer`)
    (:`True`
      (`/Game/ModsShared/AmunetDungeonAssets/Interfaces/ADA_I_TriggerController.UnregisterTriggerTarget` (stale `self.ReceiveBeginPlay` _output_get) self (`self.TriggerName`)))))

(event `InteractableInterface.InteractableActivate`
  (params (Component :type "PrimitiveComponent Object Reference") (Instigator :type "PlayerController Object Reference") (HitIndex :type Integer) (TriggeredFromRadialWheel :type Boolean))
  ;[1 0.5 0.5] (Server) ActivateTrigger
  (`Timeline|Timeline_1` :!via `PlayFromStart` :!label _label
    (:`Trigger`
      (`self.FireProjectile` (`self.InitialLocationLeft`))
      (`self.FireProjectile` (`self.InitialLocationRight`)))))

(event `/Game/ModsShared/AmunetDungeonAssets/Interfaces/ADA_I_TriggerTarget.ActivateTrigger`
  (params (Value :type Integer) (Component :type "PrimitiveComponent Object Reference") (Instigator :type "Controller Object Reference") (HitIndex :type Integer))
  ;[1 0.5 0.5] (Server) ActivateTrigger
  (goto _label :!via `PlayFromStart`))

(event `InteractableInterface.InteractableMenu`
  (params (RadialMenu :type "RadialMenu Object Reference") (HitIndex :type Integer))
  ;[0.5 1 1] (Client) Handle Menu Item
  (`parent.InteractableMenu` RadialMenu HitIndex)
  (if (`self.IsOwner` (`Controller.K2_GetPawn` (`UserWidget.GetOwningPlayer` RadialMenu)))
    (bind _returnvalue (`RadialMenu.AddItem` RadialMenu "ADA Config" (`/Game/Systems/Building/BuildingFunctionLibrary.GetBuildableObjectName` self) "/Game/Mods/AmunetDungeonAssets/UI/T_icon_edit.T_icon_edit" "None" 0))
    (add `RadialMenuEntry.SignalClicked` _returnvalue (delegate `ClientClickedEdit`))))

(event `ClientClickedEdit`
  (params (menuEntry :type "RadialMenuEntry Object Reference"))
  ;[0.5 1 1] (Client) Handle Menu Item
  (`self.ClientLoadPopup`))

(event `ClientLoadPopup`
  ;[0.5 1 1] (Client) Trigger Configure
  (bind _returnvalue (`GUIModuleController.ActivateModule` (`GUIModuleController.GetGUIModuleController`) "TriggerConfig" true false))
  (bind _asw_ada_config_trigger (cast `/Game/Mods/AmunetDungeonAssets/UI/W_ADA_ConfigTrigger` _returnvalue))
  (`/Game/Mods/AmunetDungeonAssets/UI/W_ADA_ConfigTrigger.ConfigTrigger` _asw_ada_config_trigger self (`self.TriggerName`) true "" false 0 false 0 false 0 false 0 false 0 false 0 false 0.0 false 0.0 false (`self.DynamicDamage`) true 0 false "" false))

(event `/Game/ModsShared/AmunetDungeonAssets/Interfaces/ADA_I_TriggerTarget.ConfigTrigger`
  (params (Name :type String) (NameSub :type String) (ValueTrigger :type Integer) (ValueUp :type Integer) (ValueDown :type Integer) (ValueMask :type Integer) (ValueItemId :type Integer) (ValueItemQuantity :type Integer) (ValueDelay :type "Float (single-precision)") (ValueSize :type "Float (single-precision)") (ValueDamage :type "Float (single-precision)") (ValueVariant :type Integer) (ValueSequence :type String))
  ;[1 0.5 0.5] (Server) Trigger Configure
  (`/Game/ModsShared/AmunetDungeonAssets/Interfaces/ADA_I_TriggerController.UpdateTriggerTarget` (`self.ModController`) self (`self.TriggerName`) Name)
  (set `self.TriggerName` Name)
  (set `self.DynamicDamage` ValueDamage)
  (`PersistenceComponent.SetDirty` (`self.ConanBuildingPersistence`) true 5.0))

(fn `OnRep_ProjectileDamage`
  (`self.SetDamage` (`self.DynamicDamage`)))

(fn `SetDamage`
  (params (Damage :type "Float (double-precision)"))
  (set `self.ProjectileAttackData` (`|MakeArray` (make `/Game/Systems/Combat/STR_AttackData` "/Game/Systems/Progression/DmgTypeHealth_BP.DmgTypeHealth_BP_C" Damage))))

(fn `UserConstructionScript`
  (`parent.UserConstructionScript`))