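; Buildable Conan spike trap for dungeon building, fired by overlap when its trigger name is empty, or by a matching named trigger.
; Server registers it with the ModController, applies configurable health plus fixed stamina and concussive damage to overlapping actors, then resets after a delay.
; Multicast timelines animate the instanced spikes with sound, while OnRep IsSet syncs their position.
; Owners set name and damage through a radial-menu popup, marking persistence dirty.
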(event `self.ReceiveBeginPlay`
  ;[1 1 0.5] (Both) BeginPlay
  (`parent.ReceiveBeginPlay`)
  (`self.OnRep_IsSet`)
  (if (`KismetSystemLibrary.IsServer`)
    (if (not (== (`KismetMathLibrary.MakeVector` 0.0) (`self.K2_GetActorLocation` self)))
      (bind _outactors (`GameplayStatics.GetAllActorsOfClass` "/Game/Mods/AmunetDungeonAssets/AmunetDungeonAssets_ModController.AmunetDungeonAssets_ModController_C"))
      (bind _output_get (set `self.ModController` (`KismetArrayLibrary.Array_Get` _outactors)))
      (message `/Game/Mods/AmunetDungeonAssets/ADA_TriggerInterface.RegisterTrigger` _output_get self))))

(event `self.ReceiveEndPlay`
  (params (EndPlayReason :type "EEndPlayReason Enum" :default "Destroyed"))
  (bind _modcontroller (`self.ModController`))
  ;[1 1 0.5] (Both) BeginPlay
  (`parent.ReceiveEndPlay` EndPlayReason)
  (`/Game/Systems/BP_MacroGlobal.IsValid+Branch` _modcontroller (`KismetSystemLibrary.IsServer`)
    (:`True`
      (message `/Game/Mods/AmunetDungeonAssets/ADA_TriggerInterface.UnregisterTrigger` _modcontroller self))))

(event `self.TrapTriggerBox.OnComponentBeginOverlap`
  (params (OverlappedComponent :type "PrimitiveComponent Object Reference") (OtherActor :type "Actor Object Reference") (OtherComp :type "PrimitiveComponent Object Reference") (OtherBodyIndex :type Integer) (bFromSweep :type Boolean) (SweepResult :type "HitResult Structure (by ref)"))
  ;[1 0.5 0.5] (Server) OnOverlap or ActivateTrigger
  (`/Game/Systems/BP_MacroGlobal.And+Branch` (== (`self.TriggerName`) "") (and (`KismetSystemLibrary.IsServer`) (`self.IsSet`))
    (:`True`
      (`self.MulticastTrapFire` :!label _label)
      (`KismetSystemLibrary.Delay` 1.5)
      (`self.MulticastTrapReset`))))

(event `MulticastTrapFire`
  ;[1 0.6413 0.1882] Trigger visuals
  (if (`KismetSystemLibrary.IsServer`)
    (set `self.IsSet` false)
    (for _array_element (`PrimitiveComponent.GetOverlappingActors` (`self.TrapTriggerBox`) null)
      (`GameplayStatics.ApplyDamage` _array_element (`self.DynamicDamage`) null self "/Game/Systems/Progression/DmgTypeHealth_BP.DmgTypeHealth_BP_C")
      (`GameplayStatics.ApplyDamage` _array_element 50.0 null self "/Game/Systems/Progression/DmgTypeStamina_BP.DmgTypeStamina_BP_C")
      (`GameplayStatics.ApplyDamage` _array_element 50.0 null self "/Game/Systems/Progression/DmgTypeConcusive_BP.DmgTypeConcusive_BP_C")
      (`PrimitiveComponent.SetCollisionEnabled` (`self.TrapTriggerBox`) "NoCollision")))
  (`GameplayStatics.PlaySoundAtLocation` "/Game/Sound/SFX/Doors/Traps/Spike_Trap/spike_trap_activate_multiple_Cue.spike_trap_activate_multiple_Cue" (`self.K2_GetActorLocation` self) (struct) 1.0 1.0)
  (bind (_direction _alpha) (`Timeline|TrapFireTimeline` :!via `PlayFromStart`)
    (:`Update`
      (`SceneComponent.K2_SetRelativeLocation` (`self.InstancedStaticMesh`) (`KismetMathLibrary.MakeVector` 0.0 0.0 _alpha) false false))))

(event `/Game/Mods/AmunetDungeonAssets/ADA_TriggerInterface.ActivateTrigger`
  (params (Name :type String) (Value :type Integer) (Component :type "PrimitiveComponent Object Reference") (Instigator :type "Controller Object Reference") (HitIndex :type Integer))
  ;[1 0.5 0.5] (Server) OnOverlap or ActivateTrigger
  (`/Game/Systems/BP_MacroGlobal.And+Branch` (== (`self.TriggerName`) Name) (`self.IsSet`)
    (:`True`
      (goto _label))))

(event `MulticastTrapReset`
  ;[0.02499 0.09524 0.16] Reset visuals
  (bind (_direction _alpha) (`Timeline|TrapResetTimeline` :!via `PlayFromStart`)
    (:`Update`
      (`SceneComponent.K2_SetRelativeLocation` (`self.InstancedStaticMesh`) (`KismetMathLibrary.MakeVector` 0.0 0.0 _alpha) false false))
    (:`Finished`
      (if (`KismetSystemLibrary.IsServer`)
        (set `self.IsSet` true)
        (`PrimitiveComponent.SetCollisionEnabled` (`self.TrapTriggerBox`) "QueryOnly")))
    (:`MoveDownEvent`
      (`GameplayStatics.PlaySoundAtLocation` "/Game/Sound/SFX/Doors/Traps/Spike_Trap/spike_trap_retract_2_Cue.spike_trap_retract_2_Cue" (`self.K2_GetActorLocation` self)))))

(event `InteractableInterface.InteractableMenu`
  (params (RadialMenu :type "RadialMenu Object Reference") (HitIndex :type Integer))
  ;[0.5 1 1] (Client) Handle Menu Item
  (`parent.InteractableMenu` RadialMenu HitIndex)
  (if (`self.IsOwner` (`Controller.K2_GetPawn` (`UserWidget.GetOwningPlayer` RadialMenu)))
    (bind _returnvalue (`RadialMenu.AddItem` RadialMenu "ADA Config" (`/Game/Characters/SurvivalFunctionLibrary.GetBuildableObjectName` self) "/Game/Mods/AmunetDungeonAssets/UI/T_icon_edit.T_icon_edit" "None" 0))
    (add `RadialMenuEntry.SignalClicked` _returnvalue (delegate `ClientClickedEdit`))))

(event `ClientClickedEdit`
  (params (menuEntry :type "RadialMenuEntry Object Reference"))
  ;[0.5 1 1] (Client) Handle Menu Item
  (`self.ClientLoadPopup`))

(event `ClientLoadPopup`
  ;[0.5 1 1] (Client) Trigger Configure
  (bind _returnvalue (`GUIModuleController.ActivateModule` (`GUIModuleController.GetGUIModuleController`) "TriggerConfig" true false))
  (bind _asw_ada_config_trigger (cast `/Game/Mods/AmunetDungeonAssets/UI/W_ADA_ConfigTrigger` _returnvalue))
  (`/Game/Mods/AmunetDungeonAssets/UI/W_ADA_ConfigTrigger.ConfigTrigger` _asw_ada_config_trigger self (`self.TriggerName`) true "" false 0 false 0 false 0 false 0 false 0 false 0 false 0.0 false 0.0 false (`self.DynamicDamage`) true 0 false "" false))

(event `/Game/Mods/AmunetDungeonAssets/ADA_TriggerInterface.ConfigTrigger`
  (params (Name :type String) (NameSub :type String) (ValueTrigger :type Integer) (ValueUp :type Integer) (ValueDown :type Integer) (ValueMask :type Integer) (ValueItemId :type Integer) (ValueItemQuantity :type Integer) (ValueDelay :type "Float (single-precision)") (ValueSize :type "Float (single-precision)") (ValueDamage :type "Float (single-precision)") (ValueVariant :type Integer) (ValueSequence :type String))
  ;[1 0.5 0.5] (Server) Trigger Configure
  (set `self.TriggerName` Name)
  (set `self.DynamicDamage` ValueDamage)
  (`PersistenceComponent.SetDirty` (`self.ConanBuildingPersistence`) true 5.0))

(fn `CanBePlaced`
  (params (AttachTo :type "BuildableBase Object Reference") (InstanceIndex :type Integer))
  (returns (FailedMessage :type String) (ReturnValue :type "ECanBePlacedResult Enum"))
  (bind (_failedmessage _returnvalue) (`parent.CanBePlaced` AttachTo InstanceIndex))
  (return _failedmessage _returnvalue))

(fn `InteractableGetUIModuleName`
  (returns (ReturnValue :type Name))
  (return "None"))

(fn `OnRep_IsSet`
  (`SceneComponent.K2_SetRelativeLocation` (`self.InstancedStaticMesh`) (select `bool` (`self.IsSet`) :`true` (`self.InitialLocation`)) false false))

(fn `UserConstructionScript`
  (`parent.UserConstructionScript`))